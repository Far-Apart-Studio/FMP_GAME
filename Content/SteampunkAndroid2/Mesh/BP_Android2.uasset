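; BP_Android2 is a player-controllable steampunk android character with modular coat, suit, hat and weapon parts.
; The construction script slaves each part to the main Mesh through Master Pose Component and toggles its visibility from a boolean variable.
; The event graph maps mouse axes to controller yaw and pitch, and movement axes to input along the control rotation's forward and right vectors.
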(event EventBeginPlay)

(event Collision|EventActorBeginOverlap
  (params (OtherActor :type Actor%20Object%20Reference)))

(event EventTick
  (params (DeltaSeconds :type Float%20%28single-precision%29)))

(event Input|AxisEvents|InputAxisTurnRight/LeftMouse
  (params (AxisValue :type Float%20%28single-precision%29))
  (Pawn|Input|AddControllerYawInput AxisValue))

(event Input|AxisEvents|InputAxisLookUp/DownMouse
  (params (AxisValue :type Float%20%28single-precision%29))
  (Pawn|Input|AddControllerPitchInput AxisValue))

(event Input|AxisEvents|InputAxisMoveForward/Backward
  (params (AxisValue :type Float%20%28single-precision%29))
  (Pawn|Input|AddMovementInput (Math|Vector|GetForwardVector (Pawn|GetControlRotation :!class /Script/Engine.Pawn)) AxisValue false))

(event Input|AxisEvents|InputAxisMoveRight/Left
  (params (AxisValue :type Float%20%28single-precision%29))
  (Pawn|Input|AddMovementInput (Math|Vector|GetRightVector (Pawn|GetControlRotation :!class /Script/Engine.Pawn)) AxisValue false))

(fn ConstructionScript
  (Class|SkinnedMeshComponent|SetMasterPoseComponent (Variables|Default|GetCoat) (Variables|Character|GetMesh) false)
  (Utilities|FlowControl|Sequence
    (:then_0
      (Rendering|SetVisibility (Variables|Default|GetCoat) (Variables|Default|GetCoatVis) false))
    (:then_1
      (Rendering|SetVisibility (Variables|Default|GetSuit) (Variables|Default|GetSuitVis) false))
    (:then_2
      (Rendering|SetVisibility (Variables|Default|GetHat) (Variables|Default|GetHatVis) false))
    (:then_3
      (Rendering|SetVisibility (Variables|Default|GetWeapon) (Variables|Default|GetGun) false))))