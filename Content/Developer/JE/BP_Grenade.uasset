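; BP_Grenade is a developer-folder grenade Blueprint that only logs equip state, with no throw or explosion logic.
; On BeginPlay it binds handlers to the apply and clear object-action dispatchers, apparently its equip and unequip events.
; Equip prints the owner's replicated sprint state, sprint multiplier and maximum velocity from PW_CharacterMovementComponent.
; Unequip prints only a debug message.
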(event Custom|OnEquip
  (params (characterOwner :type PW%20Character%20Object%20Reference))
  (bind _returnvalue (Actor|GetComponentbyClass characterOwner "/Script/PROJECT_WEST.PW_CharacterMovementComponent"))
  (bind __replicatedmovementdata (Variables|/Script/PROJECT_WEST.PW_CharacterMovementComponent|Get_replicatedMovementData _returnvalue))
  (bind (_issprinting _sprintmultiplier _maximumvelocity) (Utilities|Struct|BreakReplicatedMovementData __replicatedmovementdata))
  (Development|PrintString "Equip")
  (Development|PrintString (Utilities|String|ToString(Boolean) _issprinting))
  (Development|PrintString (Utilities|String|ToString(Float) _sprintmultiplier))
  (Development|PrintString (Utilities|String|ToString(Float) _maximumvelocity)))

(event Custom|OnUnEquip
  (params (characterOwner :type PW%20Character%20Object%20Reference))
  (Development|PrintString "Un Equip"))

(event EventBeginPlay
  (EventDispatchers|BindEventtoOnApplyObjectActions (EventDispatchers|CreateEvent :!event Custom|OnEquip))
  (EventDispatchers|AssignOnClearObjectActions (EventDispatchers|CreateEvent :!event Custom|OnUnEquip)))

(fn ConstructionScript)