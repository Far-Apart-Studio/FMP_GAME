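; BP_WeaponLeverAction is a lever-action weapon Blueprint that extends a parent weapon class with its own firing response.
; On fire, it runs the parent logic, casts its owner to BP_Character, calls a slowed montage playback with no montage asset set, and emits noise at the character's location with a limited range.
; BeginPlay, reload and construction only forward to the parent, and Tick is disabled.
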(event EventBeginPlay
  (|CallParentFunction))

(event EventTick
  (params (DeltaSeconds :type Float%20%28single-precision%29))
  (|CallParentFunction DeltaSeconds) ; This node is disabled and will not be called.\nDrag off pins to build functionality.
)

(event EventOnWeaponBeginReload
  (|CallParentFunction))

(event EventOnWeaponFire
  (|CallParentFunction)
  (bind _asbp_character (Utilities|Casting|CastToBP_Character (Components|GetOwner)))
  (Animation|PlayAnimMontage _asbp_character 0 0.7 "None")
  (Class|Actor|MakeNoise 1.0 _asbp_character (Transformation|GetActorLocation _asbp_character) 6e+03 "None"))

(fn ConstructionScript
  (|CallParentFunction))

(fn ReceiveActorBeginOverlap
  (params (OtherActor :type Actor%20Object%20Reference)))