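; Pistol weapon Blueprint that handles the sound, visual and animation feedback for firing, reloading and hits.
; BeginPlay caches effects from WeaponVisualData and binds the weapon hit event.
; Fire and reload pass through Server then Multi events; firing plays sound, a revolver montage on the owning BP_Character, spawns an attached emitter and emits noise.
; The hit handler spawns a bullet tracer system with beam endpoints taken from the hit result.
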(event Custom|Server
  (CallFunction|Multi))

(event Custom|Multi
  (Audio|SpawnSoundAttached (Variables|Default|GetWeaponFireSound) (Variables|Default|Get_muzzleLocation) "None" "0, 0, 0" "0, 0, 0" "KeepRelativeOffset" false 1.0 1.0 0.0 0 0)
  (Effects|SpawnEmitterAttached 0 (Variables|Default|Get_muzzleLocation) "None" "0, 0, 0" "0, 0, 0" "0.100000,0.100000,0.100000")
  (bind _asbp_character (Utilities|Casting|CastToBP_Character (Components|GetOwner)))
  (Animation|PlayAnimMontage _asbp_character "/Game/Project_West/Assets/Animations/Character_Animations/Revolver_Animations/Shooting_Anim/AM_RevolverShoot.AM_RevolverShoot" 0.7 "None")
  (Class|Actor|MakeNoise 1.0 _asbp_character (Transformation|GetActorLocation _asbp_character) 0.0 "None"))

(event Custom|OnHit
  (params (HitResult :type Hit%20Result%20Structure))
  (bind (_bblockinghit _binitialoverlap _time _distance _location _impactpoint _normal _impactnormal _physmat _hitactor _hitcomponent _hitbonename _bonename _hititem _elementindex _faceindex _tracestart _traceend) (Collision|BreakHitResult HitResult))
  (bind _returnvalue (Niagara|SpawnSystematLocation "/Game/Project_West/Assets/Art/VFX/BulletTracer/FXS_BulletTracer.FXS_BulletTracer" (Variables|/Script/Engine.SceneComponent|GetRelativeLocation (Variables|Default|Get_muzzleLocation))))
  (Effects|Components|ParticleSystem|SetVectorParameter _returnvalue "BeamEnd" _tracestart)
  (if _bblockinghit
    (Effects|Components|ParticleSystem|SetVectorParameter _returnvalue "BeamStart" _tracestart)
    (else
      (Effects|Components|ParticleSystem|SetVectorParameter _returnvalue "BeamStart" _traceend))))

(event Custom|ReloadServer
  (CallFunction|ReloadMulti))

(event Custom|ReloadMulti
  (Audio|PlaySoundatLocation (Variables|Default|GetWeaponReloadSound) (Transformation|GetWorldLocation (Variables|Default|Get_muzzleLocation)) "0, 0, 0" 1.0 1.0 0.0 0 0 0 0))

(event EventBeginPlay
  (bind __weaponvisualdata (Variables|Default|Get_weaponVisualData))
  (|CallParentFunction)
  (Variables|Default|SetWeaponFireSound (Variables|/Script/PROJECT_WEST.PW_WeaponVisualData|Get_fireSound __weaponvisualdata))
  (Variables|Default|SetWeaponReloadSound (Variables|/Script/PROJECT_WEST.PW_WeaponVisualData|Get_reloadSound __weaponvisualdata))
  (Variables|Default|SetWeaponMuzzleFlash (Variables|/Script/PROJECT_WEST.PW_WeaponVisualData|Get_muzzleFlash __weaponvisualdata))
  (EventDispatchers|BindEventtoOnWeaponHit (EventDispatchers|CreateEvent :!event Custom|OnHit)))

(event Collision|EventActorBeginOverlap
  (params (OtherActor :type Actor%20Object%20Reference))
  (|CallParentFunction OtherActor) ; This node is disabled and will not be called.\nDrag off pins to build functionality.
)

(event EventTick
  (params (DeltaSeconds :type Float%20%28single-precision%29))
  (|CallParentFunction DeltaSeconds) ; This node is disabled and will not be called.\nDrag off pins to build functionality.
)

(event EventOnWeaponFire
  (CallFunction|Server))

(event EventOnWeaponBeginReload
  (CallFunction|ReloadServer))

(fn ConstructionScript
  (|CallParentFunction))