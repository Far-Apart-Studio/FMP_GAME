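; Bolt-action sniper rifle weapon Blueprint that extends parent weapon events with character animations and a scope view.
; Firing routes through FireServer to FireMulti, which plays an aim or hip shot montage, emits noise, then rechambers the bolt after a delay.
; Aiming briefly waits, rechecks the aim state, then enables the character's scope and hides the rifle from its owner; hipfire reverses this.
; Reload plays a character montage.
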(event Custom|FireServer
  ;[1 1 1] Shoot
  (CallFunction|FireMulti))

(event Custom|FireMulti
  ;[1 1 1] Shoot
  (bind _asbp_character (Utilities|Casting|CastToBP_Character (Components|GetOwner)))
  (if (Variables|/Game/Project_West/Game/Character/Blueprints/BP_Character.BP_Character_C|GetAiming _asbp_character)
    (Animation|PlayAnimMontage _asbp_character "/Game/Project_West/Temp/TB/CharAnimsTemp/WeaponAnims/AM_RifleAimShoot.AM_RifleAimShoot" 1.0 "None")
    (else
      (Animation|PlayAnimMontage _asbp_character "/Game/Project_West/Temp/TB/CharAnimsTemp/WeaponAnims/AM_RifleHipShoot.AM_RifleHipShoot" 1.0 "None")))
  (Class|Actor|MakeNoise 1.0 _asbp_character (Transformation|GetActorLocation _asbp_character) 6e+03 "None")
  (Utilities|FlowControl|Delay 0.5)
  (Components|Animation|PlayAnimation (Variables|Default|Get_itemMesh) "/Game/Project_West/Temp/TB/CharAnimsTemp/WeaponAnims/AM_BoltActionRechamber.AM_BoltActionRechamber" false))

(event EventBeginPlay
  (|CallParentFunction))

(event EventHipfireMode
  ;[1 1 1] Scoping
  (|CallParentFunction)
  (bind _asbp_character (Utilities|Casting|CastToBP_Character (Components|GetOwner)))
  (Default|DisableScope _asbp_character)
  (Class|PrimitiveComponent|SetOwnerNoSee (Variables|Default|Get_itemMesh) false))

(event EventUnequip
  (params (WeaponObject :type PW%20Weapon%20Object%20Object%20Reference))
  ;[1 1 1] Equip/Unequip
  (|CallParentFunction 0)
  (Variables|/Script/Engine.SkeletalMeshComponent|SetbPauseAnims (Variables|Default|Get_itemMesh) true))

(event EventTick
  (params (DeltaSeconds :type Float%20%28single-precision%29))
  (|CallParentFunction DeltaSeconds) ; This node is disabled and will not be called.\nDrag off pins to build functionality.
)

(event EventOnWeaponFireModeAimEvent
  (bind __itemmesh (Variables|Default|Get_itemMesh))
  ;[1 1 1] Scoping
  (|CallParentFunction)
  (bind _asbp_character (Utilities|Casting|CastToBP_Character (Components|GetOwner)))
  (Utilities|FlowControl|Delay 0.25)
  (if (Variables|/Game/Project_West/Game/Character/Blueprints/BP_Character.BP_Character_C|GetAiming _asbp_character)
    (Default|EnableScope _asbp_character)
    (Class|PrimitiveComponent|SetOwnerNoSee __itemmesh true)
    (else
      (bind _asbp_character_2 (Utilities|Casting|CastToBP_Character (Components|GetOwner)))
      (Default|DisableScope _asbp_character_2)
      (Class|PrimitiveComponent|SetOwnerNoSee __itemmesh false))))

(event EventOnWeaponBeginReload
  ;[1 1 1] Reloading
  (|CallParentFunction))

(event EventReloadServer
  ;[1 1 1] Reloading
  (|CallParentFunction))

(event EventReloadMulti
  ;[1 1 1] Reloading
  (|CallParentFunction)
  (bind _asbp_character (Utilities|Casting|CastToBP_Character (Components|GetOwner)))
  (Animation|PlayAnimMontage _asbp_character "/Game/Project_West/Assets/Animations/Weapon_Animations/Revolver_Animations/Reload_Anim/AM_WeaponReload.AM_WeaponReload" 1.0 "None"))

(event EventEquip
  (params (WeaponObject :type PW%20Weapon%20Object%20Object%20Reference))
  ;[1 1 1] Equip/Unequip
  (|CallParentFunction 0)
  (Variables|/Script/Engine.SkeletalMeshComponent|SetbPauseAnims (Variables|Default|Get_itemMesh) false))

(event EventOnWeaponFire
  ;[1 1 1] Shoot
  (|CallParentFunction)
  (CallFunction|FireServer))

(fn ConstructionScript
  (|CallParentFunction))

(fn ReceiveActorBeginOverlap
  (params (OtherActor :type Actor%20Object%20Reference)))