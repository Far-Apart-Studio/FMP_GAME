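; Shotgun weapon Blueprint that specializes a parent weapon class, adding firing feedback and HUD presentation.
; On fire, it runs the parent logic, plays a slowed montage on the owning BP_Character and emits AI-audible noise at that character's location.
; Equip and unequip toggle the weapon widget's visibility and set its shotgun icon and name.
; Reload events only forward to the parent.
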(event EventBeginPlay
  (|CallParentFunction))

(event EventOnWeaponBeginReload
  ;[1 1 1] Reloading
  (|CallParentFunction))

(event EventOnEquip
  (params (characterOwner :type PW%20Character%20Object%20Reference))
  (bind _weaponwidget (Variables|Default|GetWeaponWidget))
  (|CallParentFunction characterOwner)
  (Widget|SetVisibility (Variables|Default|GetWeaponWidget) "Visible")
  (Appearance|SetBrushfromTexture (Variables|/Game/Project_West/Temp/NP/UI/WB_LoadoutSlot.WB_LoadoutSlot_C|GetCurrentWeapon_Icon _weaponwidget) "/Game/Project_West/Assets/Art/UI/Icons/T_ShotgunIcon.T_ShotgunIcon" false)
  (Appearance|SetBrushfromTexture (Variables|/Game/Project_West/Temp/NP/UI/WB_LoadoutSlot.WB_LoadoutSlot_C|GetCurrentWeaponShadow_Icon _weaponwidget) "/Game/Project_West/Assets/Art/UI/Icons/T_ShotgunIcon.T_ShotgunIcon" false)
  (Variables|/Script/UMG.TextBlock|SetText (Variables|/Game/Project_West/Temp/NP/UI/WB_LoadoutSlot.WB_LoadoutSlot_C|GetGunName _weaponwidget) "Shotgun"))

(event EventOnUnequip
  (params (characterOwner :type PW%20Character%20Object%20Reference))
  (bind _weaponwidget (Variables|Default|GetWeaponWidget))
  (|CallParentFunction characterOwner)
  (Widget|SetVisibility (Variables|Default|GetWeaponWidget) "Hidden")
  (Appearance|SetBrushfromTexture (Variables|/Game/Project_West/Temp/NP/UI/WB_LoadoutSlot.WB_LoadoutSlot_C|GetCurrentWeapon_Icon _weaponwidget) "/Game/Project_West/Assets/Art/UI/Icons/T_ShotgunIcon.T_ShotgunIcon" false)
  (Appearance|SetBrushfromTexture (Variables|/Game/Project_West/Temp/NP/UI/WB_LoadoutSlot.WB_LoadoutSlot_C|GetCurrentWeaponShadow_Icon _weaponwidget) "/Game/Project_West/Assets/Art/UI/Icons/T_ShotgunIcon.T_ShotgunIcon" false)
  (Variables|/Script/UMG.TextBlock|SetText (Variables|/Game/Project_West/Temp/NP/UI/WB_LoadoutSlot.WB_LoadoutSlot_C|GetGunName _weaponwidget) "Shotgun"))

(event EventTick
  (params (DeltaSeconds :type Float%20%28single-precision%29))
  (|CallParentFunction DeltaSeconds) ; This node is disabled and will not be called.\nDrag off pins to build functionality.
)

(event EventReloadServer
  ;[1 1 1] Reloading
  (|CallParentFunction))

(event EventReloadMulti
  ;[1 1 1] Reloading
  (|CallParentFunction))

(event EventOnWeaponFire
  (|CallParentFunction)
  (bind _asbp_character (Utilities|Casting|CastToBP_Character (Components|GetOwner)))
  (Animation|PlayAnimMontage _asbp_character 0 0.7 "None")
  (Class|Actor|MakeNoise 1.0 _asbp_character (Transformation|GetActorLocation _asbp_character) 6e+03 "None"))

(fn ConstructionScript
  (|CallParentFunction))

(fn ReceiveActorBeginOverlap
  (params (OtherActor :type Actor%20Object%20Reference)))