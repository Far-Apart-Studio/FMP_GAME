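; Base weapon Blueprint handling the cosmetic and owner-feedback side of firing, reloading, aiming and equipping.
; BeginPlay binds weapon delegates and caches effects from WeaponVisualData, with fire, reload and aim relayed through server-to-multicast events.
; Successful shots multicast a Niagara beam tracer and impact effect, while hits on living health-component actors trigger the owner's hitmarker.
; Aiming starts camera wobble, switching to a hold-breath shake after a delay, and equip changes update BP_Character's selected weapon.
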(event Custom|MulticastFire
  ;[1 1 1] WeaponFireEvent
  (Audio|SpawnSoundAttached (Variables|Default|GetWeaponFireSound) (Variables|Default|Get_muzzleLocation) "None" "0, 0, 0" "0, 0, 0" "KeepRelativeOffset" false 1.0 1.0 0.0 0 0)
  (bind _returnvalue (Class|PWWeaponVisualData|GetMuzzleFlashNiagara (Variables|Default|Get_weaponVisualData)))
  (Niagara|SpawnSystemAttached _returnvalue (Variables|Default|Get_muzzleLocation) "None" "0, 0, 0" "0, 0, 0" "KeepRelativeOffset" false))

(event Custom|ServerFire
  ;[1 1 1] WeaponFireEvent
  (CallFunction|MulticastFire))

(event Custom|HipfireMode
  ;[1 1 1] AimAnimations
  (CameraShake|StopAllCameraShakes (Variables|Default|GetCameraShakeSource) true)
  (CallFunction|HipfireServer))

(event Custom|AImMulticast
  ;[1 1 1] AimAnimations
  (bind _asbp_character (Utilities|Casting|CastToBP_Character (Components|GetOwner)))
  (Variables|/Game/Project_West/Game/Character/Blueprints/BP_Character.BP_Character_C|SetAiming _asbp_character true))

(event Custom|HipfireMulticast
  ;[1 1 1] AimAnimations
  (bind _asbp_character (Utilities|Casting|CastToBP_Character (Components|GetOwner)))
  (Variables|/Game/Project_West/Game/Character/Blueprints/BP_Character.BP_Character_C|SetAiming _asbp_character false))

(event Custom|HipfireServer
  ;[1 1 1] AimAnimations
  (CallFunction|HipfireMulticast))

(event Custom|AimServer
  ;[1 1 1] AimAnimations
  (CallFunction|AImMulticast))

(event Custom|HitActor
  (params (HitResult :type Hit%20Result%20Structure))
  (bind _hitactor (Collision|BreakHitResult HitResult))
  (bind _returnvalue (Actor|GetComponentbyClass _hitactor "/Script/PROJECT_WEST.PW_HealthComponent"))
  ;[1 1 1] WeaponFireEvent
  (Utilities|IsValid _returnvalue
    (:Is%20Valid
      (if (not (<= (Variables|/Script/PROJECT_WEST.PW_HealthComponent|Get_currentHealth _returnvalue) 0.0))
        (bind _asbp_character (Utilities|Casting|CastToBP_Character (Components|GetOwner)))
        (Default|ActivateHitmarker _asbp_character)))))

(event Custom|Equip
  (params (WeaponObject :type PW%20Weapon%20Object%20Object%20Reference))
  ;[1 1 1] Equip/Unequip Event
  (bind _asbp_character (Utilities|Casting|CastToBP_Character (Components|GetOwner)))
  (Default|SelectedWeapon _asbp_character (Variables|Default|GetWeaponID)))

(event Custom|Unequip
  (params (WeaponObject :type PW%20Weapon%20Object%20Object%20Reference))
  ;[1 1 1] Equip/Unequip Event
  (bind _asbp_character (Utilities|Casting|CastToBP_Character (Components|GetOwner)))
  (Default|SelectedWeapon _asbp_character))

(event Custom|On%20Successful%20Fire
  (params (HitResult :type Hit%20Result%20Structure) (StartPoint :type Vector) (EndPoint :type Vector))
  (bind (_bblockinghit _binitialoverlap _time _distance _location _impactpoint _normal _impactnormal _physmat _hitactor _hitcomponent _hitbonename _bonename _hititem _elementindex _faceindex _tracestart _traceend) (Collision|BreakHitResult HitResult))
  ;[1 1 1] WeaponFireTracer
  (CallFunction|MulticastFireTracer _impactpoint _tracestart _traceend _bblockinghit))

(event Custom|ReloadServer
  ;[1 1 1] WeaponReload
  (CallFunction|ReloadMulti))

(event Custom|ReloadMulti
  ;[1 1 1] WeaponReload
  (Audio|SpawnSoundAttached (Variables|Default|GetWeaponReloadSound) (Variables|Default|Get_muzzleLocation) "None" "0, 0, 0" "0, 0, 0" "KeepRelativeOffset" false 1.0 1.0 0.0 0 0))

(event Custom|On%20Weapon%20Fire
  ;[1 1 1] WeaponFireEvent
  (Camera|PlayWorldCameraShake (Variables|Default|GetCam%20Shake%20Fire) (Transformation|GetActorLocation) 2e+02 2e+02)
  (CallFunction|ServerFire))

(event Custom|On%20Weapon%20Stop%20Fire
  ;[1 1 1] WeaponFireEvent
)

(event Custom|On%20Weapon%20Begin%20Reload
  ;[1 1 1] WeaponReload
  (CallFunction|ReloadServer))

(event Custom|Multicast%20Fire%20Tracer
  (params (ImpactPoint :type Vector) (TraceStart :type Vector) (TraceEnd :type Vector) (BlockingHit :type Boolean))
  (bind __muzzlelocation (Variables|Default|Get_muzzleLocation))
  (bind _returnvalue (Transformation|GetWorldLocation __muzzlelocation))
  ;[1 1 1] WeaponFireTracer
  (bind _returnvalue_2 (Class|PWWeaponVisualData|GetProjectileTracerNiagara (Variables|Default|Get_weaponVisualData)))
  (bind _returnvalue_3 (Niagara|SpawnSystematLocation _returnvalue_2 _returnvalue (Transformation|GetWorldRotation __muzzlelocation)))
  (Effects|Components|ParticleSystem|SetVectorParameter _returnvalue_3 "BeamStart" _returnvalue)
  (if BlockingHit
    (Effects|Components|ParticleSystem|SetVectorParameter _returnvalue_3 "BeamEnd" ImpactPoint)
    (Niagara|SpawnSystematLocation "/Game/Project_West/Assets/Art/VFX/Rifle/RifleImpact/FXS_RifleImpact.FXS_RifleImpact" ImpactPoint)
    (else
      (Effects|Components|ParticleSystem|SetVectorParameter _returnvalue_3 "BeamEnd" TraceEnd))))

(event Custom|OnWeaponFireModeAim_Event
  (bind _camerashakesource (Variables|Default|GetCameraShakeSource))
  ;[1 1 1] AimAnimations
  (CameraShake|Start _camerashakesource)
  (CallFunction|AimServer)
  (Utilities|FlowControl|RetriggerableDelay 6.0)
  (if (Variables|/Game/Project_West/Game/Character/Blueprints/BP_Character.BP_Character_C|GetAiming (stale Custom|AImMulticast _asbp_character))
    (Class|CameraShakeSourceComponent|StopAllCameraShakesOfType _camerashakesource "/Game/Developer/JE/Weapons/CS_SniperWobble.CS_SniperWobble_C" false)
    (CameraShakes|StartCameraShake _camerashakesource "/Game/Developer/JE/Weapons/CS_SniperHoldBreath.CS_SniperHoldBreath_C" 1.0 "CameraLocal" "0, 0, 0")))

(event EventBeginPlay
  (bind __weaponvisualdata (Variables|Default|Get_weaponVisualData))
  ;[1 1 1] Beginplay
  (EventDispatchers|AssignOnWeaponFireDelegate (EventDispatchers|CreateEvent :!event Custom|On%20Weapon%20Fire))
  (EventDispatchers|AssignOnWeaponStopFire (EventDispatchers|CreateEvent :!event Custom|On%20Weapon%20Stop%20Fire))
  (EventDispatchers|AssignOnWeaponBeginReload (EventDispatchers|CreateEvent :!event Custom|On%20Weapon%20Begin%20Reload))
  (EventDispatchers|AssignOnWeaponSuccessfulFire (EventDispatchers|CreateEvent :!event Custom|On%20Successful%20Fire))
  (Variables|Default|SetWeaponFireSound (Variables|/Script/PROJECT_WEST.PW_WeaponVisualData|Get_fireSound __weaponvisualdata))
  (Variables|Default|SetWeaponReloadSound (Variables|/Script/PROJECT_WEST.PW_WeaponVisualData|Get_reloadSound __weaponvisualdata))
  (Variables|Default|SetWeaponMuzzleFlash (Variables|/Script/PROJECT_WEST.PW_WeaponVisualData|Get_muzzleFlash __weaponvisualdata))
  (EventDispatchers|AssignOnWeaponFireModeAim (EventDispatchers|CreateEvent :!event Custom|OnWeaponFireModeAim_Event))
  (EventDispatchers|BindEventtoOnWeaponFireModeHip (EventDispatchers|CreateEvent :!event Custom|HipfireMode))
  (EventDispatchers|BindEventtoOnWeaponHit (EventDispatchers|CreateEvent :!event Custom|HitActor))
  (EventDispatchers|AssignOnWeaponEquip (EventDispatchers|CreateEvent :!event Custom|Equip))
  (EventDispatchers|AssignOnWeaponUnEquip (EventDispatchers|CreateEvent :!event Custom|Unequip)))

(fn ConstructionScript)