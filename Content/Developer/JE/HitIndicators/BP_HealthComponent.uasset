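; Health component Blueprint that shows on-screen damage feedback for hit-indicator work.
; BeginPlay binds to the global damage-received delegate, whose handler spawns a WBP_Hit widget per event, passing owner, causer, amount, duration and render threshold before it self-destructs.
; A separate OnDamageRecieved handler briefly shows a WB_PlayerHurt overlay, then removes it after a delay.
; Both handlers create widgets for player controller 0, with no check on who was damaged.
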(event Custom|OnDamageReceivedGlobal_Event
  (params (OwnerActor :type Actor%20Object%20Reference) (DamageCauser :type Actor%20Object%20Reference) (DamageCauserController :type Controller%20Object%20Reference) (DamageAmount :type Float%20%28single-precision%29))
  (bind _returnvalue (UserInterface|CreateWidget "/Game/Developer/JE/HitIndicators/WBP_Hit.WBP_Hit_C" (Game|GetPlayerController 0)))
  (Class|DamageIndicatorWidget|SetHitDetails _returnvalue (Utilities|Struct|MakeIndicateHandle OwnerActor DamageCauser DamageAmount (Variables|DamageIndicator|GetIndicateDuration) (Variables|DamageIndicator|GetRenderThreshold)))
  (UserInterface|Viewport|AddtoViewport _returnvalue 0)
  (Class|DamageIndicatorWidget|SelfDestruct _returnvalue))

(event Custom|OnDamageRecieved
  (params (OwnerActor :type Actor%20Object%20Reference) (DamageCauser :type Actor%20Object%20Reference) (DamageCauserController :type Controller%20Object%20Reference) (DamageAmount :type Float%20%28single-precision%29))
  (bind _returnvalue (UserInterface|CreateWidget "/Game/Project_West/UI/Misc/WB_PlayerHurt.WB_PlayerHurt_C" (Game|GetPlayerController 0)))
  (UserInterface|Viewport|AddtoViewport _returnvalue 0)
  (Utilities|FlowControl|Delay 2.0)
  (Widget|RemovefromParent _returnvalue))

(event EventBeginPlay
  (EventDispatchers|AssignOnDamageReceivedGlobal (delegate Custom|OnDamageReceivedGlobal_Event))
  (EventDispatchers|AssignOnDamageReceivedGlobal (EventDispatchers|CreateEvent :!event Custom|OnDamageRecieved)))