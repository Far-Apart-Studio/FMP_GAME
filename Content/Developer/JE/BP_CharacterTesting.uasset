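; BP_CharacterTesting is a developer test character Blueprint for trying out death handling, map input and game mode access.
; On BeginPlay it binds PWHealth's OnDeath to a relay event that plays the Android death animation on the mesh.
; The Map action creates the PW_Map widget through a FlipFlop, with only the first branch wired.
; The T key casts the bounty game mode directly or via a server event, with nothing after; aim-button debug prints are left unbound.
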(event Custom|Server%20Game%20Mode
  ;[1 1 1] Test
  (Utilities|Casting|CastToPW_BountyGameMode_BP (Game|GetGameMode)))

(event Custom|OnDeathEvent
  (params (DamageCauser :type Actor%20Object%20Reference) (DamageCauserController :type Controller%20Object%20Reference))
  ;[1 1 1] DeathAnimationHandling
  (CallFunction|OnDeathMulti))

(event Custom|OnAimButtonPressed_Event
  (Development|PrintString "Helloooo")
  (Development|PrintText "Hello"))

(event Custom|OnDeathMulti
  ;[1 1 1] DeathAnimationHandling
  (Components|Animation|PlayAnimation (Variables|Character|GetMesh) "/Game/ExternalAssets/SteampunkAndroid2/Animation/Anim_Android2_Death.Anim_Android2_Death" false))

(event Custom|DeathBind
  ;[1 1 1] DeathAnimationHandling
  (EventDispatchers|AssignOnDeath (Variables|Default|GetPW_Health) (delegate Custom|OnDeathEvent)))

(event EventBeginPlay
  (CallFunction|DeathBind))

(event Input|ActionEvents|InputActionMap
  (params (Key :type Key%20Structure :default "None"))
  ;[1 1 1] Map
  (:Pressed
    (Utilities|FlowControl|FlipFlop
      (:A
        (UserInterface|CreateWidget "/Game/Project_West/Game/Map/PW_Map.PW_Map_C")))))

(event Input|KeyboardEvents|T
  (params (Key :type Key%20Structure :default "None"))
  ;[1 1 1] Test
  (:Pressed
    (if (Ability|HasAuthority)
      (Utilities|Casting|CastToPW_BountyGameMode_BP (Game|GetGameMode))
      (else
        (CallFunction|ServerGameMode)))))

(fn ConstructionScript)