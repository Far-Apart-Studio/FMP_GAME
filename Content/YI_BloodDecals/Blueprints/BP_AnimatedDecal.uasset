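; Animated decal actor, apparently for blood splatter, that plays a flipbook, optionally dries, then fades out and destroys itself.
; A BeginPlay delay loop drives mask and normal time parameters on a dynamic material instance, with a speed boost for the opening splash.
; Drying gradually raises roughness and lowers metallic from the material's starting values.
; After a lifetime delay, a final loop lowers FadeOut until the actor is destroyed.
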(event EventBeginPlay
  (bind _updatetime (Variables|Default|GetUpdateTime))
  (bind _splashspeed (Variables|Default|GetSplashSpeed))
  ;[1 1 1] Frame/Update delays
  (Utilities|FlowControl|Delay _updatetime :!label _label)
  (if (>= (Variables|Default|GetTimer) (Variables|Default|GetMax_time))
    ;[1 1 1] If set to dry over time, set values to pass next branch
    (if (Variables|Default|GetDryOverTime) :!label _label_2
      (Variables|Default|SetDryOverTime false)
      (bind _returnvalue (Rendering|Material|GetScalarParameterValue (Variables|Default|GetMaterial_ToEdit) "Roughness" :!class /Script/Engine.MaterialInstanceDynamic))
      (bind _returnvalue_2 (Rendering|Material|GetScalarParameterValue (Variables|Default|GetMaterial_ToEdit) "Metallic" :!class /Script/Engine.MaterialInstanceDynamic))
      (bind _output_get (Variables|Default|SetRoughnessStart _returnvalue))
      (bind _output_get_2 (Variables|Default|SetMetallicStart _returnvalue_2))
      (Variables|Default|SetRoughness _output_get)
      (Variables|Default|SetMetallic _output_get_2)
      (goto _label_2)
      (else
        ;[1 1 1] Additional Delay Before Drying/Destroy begins
        (Utilities|FlowControl|Delay (Variables|Default|GetInitialDryDelay))
        ;[1 1 1] If set to dry, the roughness and metallic will change over time
        (if (and (< (Variables|Default|GetRoughness) (Variables|Default|GetRoughnessMax)) (> (Variables|Default|GetMetallic) (Variables|Default|GetMetallicMin))) :!label _label_3
          (Utilities|FlowControl|Delay (* (Variables|Default|GetUpdateTime) 4.0))
          (if (< (Variables|Default|GetRoughness) (Variables|Default|GetRoughnessMax))
            (bind _output_get_3 (Variables|Default|SetRoughness (+ (Variables|Default|GetRoughness) (Variables|Default|GetDryingSpeed))))
            (bind _output_get_4 (Variables|Default|SetMetallic (- (Variables|Default|GetMetallic) (Variables|Default|GetDryingSpeed)) :!label _label_4))
            (elif (> (Variables|Default|GetMetallic) (Variables|Default|GetMetallicMin))
              (goto _label_4)
              (else
                _)))
          (Rendering|Material|SetScalarParameterValue (Variables|Default|GetMaterial_ToEdit) "Roughness" _output_get_3 :!class /Script/Engine.MaterialInstanceDynamic)
          (Rendering|Material|SetScalarParameterValue (Variables|Default|GetMaterial_ToEdit) "Metallic" _output_get_4 :!class /Script/Engine.MaterialInstanceDynamic)
          (goto _label_3)
          (else
            ;[1 1 1] Fade the actor out and destroy it after a delay
            (Utilities|FlowControl|Delay (Variables|Default|GetDecalLifetime))
            (Utilities|FlowControl|Delay (* (Variables|Default|GetUpdateTime) 1.0) :!label _label_5)
            (if (> (- (Variables|Default|GetFadeOut) (Variables|Default|GetFadeOutSpeed)) 0.05)
              (bind _output_get_5 (Variables|Default|SetFadeOut (- (Variables|Default|GetFadeOut) (Variables|Default|GetFadeOutSpeed))))
              (Rendering|Material|SetScalarParameterValue (Variables|Default|GetMaterial_ToEdit) "FadeOut" _output_get_5 :!class /Script/Engine.MaterialInstanceDynamic)
              (goto _label_5)
              (else
                (Actor|DestroyActor)))))))
    (else
      ;[1 1 1] Has a dynamic material been created?
      (Variables|Default|SetTimer (+ (Variables|Default|GetTimer) (* _updatetime (Variables|Default|GetFramesPerUpdate))))
      (if (and (< (Variables|Default|GetTimer) 0.125) (> _splashspeed 0.0))
        (Variables|Default|SetTimer (+ (Variables|Default|GetTimer) _splashspeed)))
      (Utilities|IsValid (Variables|Default|GetMaterial_ToEdit)
        (:Is%20Valid
          _)
        (:Is%20Not%20Valid
          ;[1 1 1] Create Dynamic Material
          (bind _returnvalue_3 (Rendering|Material|CreateDynamicMaterialInstance (Variables|Default|GetMaterial_Instance) :!class /Script/Engine.KismetMaterialLibrary))
          (Variables|Default|SetMaterial_ToEdit _returnvalue_3)))
      ;[1 1 1] Set Flipbook Position
      (Rendering|Material|SetScalarParameterValue (Variables|Default|GetMaterial_ToEdit) "Time_Mask" (Variables|Default|GetTimer) :!class /Script/Engine.MaterialInstanceDynamic)
      (Rendering|Material|SetScalarParameterValue (Variables|Default|GetMaterial_ToEdit) "Time_Normals" (Variables|Default|GetTimer) :!class /Script/Engine.MaterialInstanceDynamic)
      (Rendering|Components|Decal|SetDecalMaterial (Variables|Decal|GetDecal) _returnvalue_3)
      (goto _label))))

(fn ConstructionScript)