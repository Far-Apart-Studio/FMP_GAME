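; Character Blueprint that handles death animation, opening the map and a bounty test key.
; On BeginPlay it binds to the PWHealth death event, which calls OnDeathMulti to play the Android death animation on the mesh.
; The Map input creates a PW_Map widget on every other press, with no removal wired.
; The T debug key calls TestModifyBountyData on the bounty game mode, going through ServerGameMode when lacking authority.
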(event Custom|Server%20Game%20Mode
  ;[1 1 1] Test
  (bind _aspw_bounty_game_mode_bp (Utilities|Casting|CastToPW_BountyGameMode_BP (Game|GetGameMode)))
  (Class|PWBountyGameMode|TestModifyBountyData _aspw_bounty_game_mode_bp)
  (Development|PrintString "Client Triggered it"))

(event Custom|OnDeathEvent
  (params (DamageCauser :type Actor%20Object%20Reference) (DamageCauserController :type Controller%20Object%20Reference))
  ;[1 1 1] DeathAnimationHandling
  (CallFunction|OnDeathMulti))

(event Custom|OnDeathMulti
  ;[1 1 1] DeathAnimationHandling
  (Components|Animation|PlayAnimation (Variables|Character|GetMesh) "/Game/ExternalAssets/SteampunkAndroid2/Animation/Anim_Android2_Death.Anim_Android2_Death" false))

(event Custom|DeathBind
  ;[1 1 1] DeathAnimationHandling
  (EventDispatchers|AssignOnDeath (Variables|Default|GetPW_Health) (delegate Custom|OnDeathEvent)))

(event EventBeginPlay
  (CallFunction|DeathBind))

(event Input|ActionEvents|InputActionMap
  (params (Key :type Key%20Structure :default "None"))
  ;[1 1 1] Map
  (:Pressed
    (Utilities|FlowControl|FlipFlop
      (:A
        (bind _returnvalue (UserInterface|CreateWidget "/Game/TB/Map/PW_Map.PW_Map_C"))
        (UserInterface|Viewport|AddtoViewport _returnvalue 0)))))

(event Input|KeyboardEvents|T
  (params (Key :type Key%20Structure :default "None"))
  ;[1 1 1] Test
  (:Pressed
    (if (Ability|HasAuthority)
      (bind _aspw_bounty_game_mode_bp (Utilities|Casting|CastToPW_BountyGameMode_BP (Game|GetGameMode)))
      (Class|PWBountyGameMode|TestModifyBountyData _aspw_bounty_game_mode_bp)
      (Development|PrintString ".....")
      (else
        (CallFunction|ServerGameMode)))))

(fn ConstructionScript)