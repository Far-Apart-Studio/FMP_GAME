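; Game mode Blueprint for a bounty mode, meant to link a spawned portal to the bounty's portal and point a lantern at it.
; On initialize complete it calls SetUpPortals and AssignPortalToLantern, but both are currently empty.
; Their disconnected nodes would find an existing BP_Teleporter, spawn another at the SpawnPointsManager's bounty portal point, connect the pair and set it as the Lantern's target.
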(event EventTick
  (params (DeltaSeconds :type Float%20%28single-precision%29)))

(event EventOnInitializeComplete
  (CallFunction|SetUpPortals)
  (CallFunction|AssignPortaltoLantern))

(fn ConstructionScript)

(fn SetUpPortals)

(fn AssignPortaltoLantern)