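; BP_Splines is a spline actor, in a testing map folder, that tiles a chosen mesh along its spline.
; The construction script adds one spline mesh component per section, with configurable collision and optionally a section length derived from actor X scale.
; StartPos and EndPosition supply length-clamped tangents, though StartPos derives its tangent from location.
; Both MustBeFullLengthMeshes branches produce the same loop range, as the subtraction is zero.
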(event EventBeginPlay)

(event Collision|EventActorBeginOverlap
  (params (OtherActor :type Actor%20Object%20Reference)))

(event EventTick
  (params (DeltaSeconds :type Float%20%28single-precision%29)))

(fn ConstructionScript
  (if (Variables|Default|GetAllowScaling?)
    (Variables|Default|SetSectionLength (* (.x (Transformation|GetActorScale3D)) 1e+02)))
  (if (Variables|Default|GetMustBeFullLengthMeshes?)
    (for _index (range 0 (- (Math|Float|Truncate (/ (Spline|GetSplineLength (Variables|Default|GetSpline)) (Variables|Default|GetSectionLength))) 0))
      (LocalVariables|SetLoop%20Index _index)
      (bind _returnvalue (AddComponent|AddSplineMeshComponent false))
      (Components|StaticMesh|SetStaticMesh _returnvalue (Variables|Default|GetSplineMesh))
      (SplineMesh|SetForwardAxis _returnvalue "X" true)
      (bind (_position _tangent) (CallFunction|StartPos (LocalVariables|GetLoop%20Index)))
      (bind (_position_2 _tangent_2) (CallFunction|EndPosition (LocalVariables|GetLoop%20Index)))
      (SplineMesh|SetStartandEnd _returnvalue _position _tangent _position_2 _tangent_2 true :!class /Script/Engine.SplineMeshComponent)
      (Collision|SetCollisionEnabled _returnvalue (Variables|Default|GetCollisionType)))
    (else
      (for _index_2 (range 0 (Math|Float|Truncate (/ (Spline|GetSplineLength (Variables|Default|GetSpline)) (Variables|Default|GetSectionLength))))
        (LocalVariables|SetLoop%20Index _index_2)
        (bind _returnvalue_2 (AddComponent|AddSplineMeshComponent false))
        (Components|StaticMesh|SetStaticMesh _returnvalue_2 (Variables|Default|GetSplineMesh))
        (SplineMesh|SetForwardAxis _returnvalue_2 "X" true)
        (bind (_position_3 _tangent_3) (CallFunction|StartPos (LocalVariables|GetLoop%20Index)))
        (bind (_position_4 _tangent_4) (CallFunction|EndPosition (LocalVariables|GetLoop%20Index)))
        (SplineMesh|SetStartandEnd _returnvalue_2 _position_3 _tangent_3 _position_4 _tangent_4 true :!class /Script/Engine.SplineMeshComponent)
        (Collision|SetCollisionEnabled _returnvalue_2 (Variables|Default|GetCollisionType))))))

(fn StartPos
  (params (Index :type Integer))
  (bind _sectionlength (Variables|Default|GetSectionLength))
  (bind _spline (Variables|Default|GetSpline))
  (bind _returnvalue (* Index _sectionlength))
  (return (Spline|GetLocationatDistanceAlongSpline _spline _returnvalue "Local") (Math|Vector|ClampVectorSize (Spline|GetLocationatDistanceAlongSpline _spline _returnvalue "Local") 0.0 (Variables|Default|GetSectionLength))))

(fn EndPosition
  (params (Index :type Integer))
  (bind _returnvalue (+ Index 1))
  (bind _sectionlength (Variables|Default|GetSectionLength))
  (bind _spline (Variables|Default|GetSpline))
  (bind _returnvalue_2 (* _returnvalue _sectionlength))
  (return (Spline|GetLocationatDistanceAlongSpline _spline _returnvalue_2 "Local") (Math|Vector|ClampVectorSize (Spline|GetTangentatDistanceAlongSpline _spline _returnvalue_2 "Local") 0.0 (Variables|Default|GetSectionLength))))