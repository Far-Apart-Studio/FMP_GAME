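; BP_Drawbridge is a drawbridge that lowers once when its ChargeAbleMechanism finishes charging.
; The charge-completed event passes through a DoOnce, then eases the bridge mesh to a -90 pitch with MoveComponentTo while a spawned sound plays.
; When the move completes, it stops that sound and plays a collapse sound and an emitter at the Scene component.
; Both interaction query functions return false.
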(event Custom|On%20Activated
  (Utilities|FlowControl|DoOnce false
    (:Completed
      (CallFunction|DropBridge))))

(event Custom|DropBridge
  (bind _drawbridge_cube_006 (Variables|Default|GetDrawbridge_Cube_006))
  (bind _scene (Variables|Default|GetScene))
  (bind _returnvalue (Transformation|GetWorldLocation _scene))
  (bind _relativerotation (Variables|/Script/Engine.SceneComponent|GetRelativeRotation _drawbridge_cube_006))
  (bind _returnvalue_2 (Audio|SpawnSoundatLocation "/Game/StarterContent/Audio/Light01.Light01" (Transformation|GetWorldLocation (Variables|Default|GetDrawbridge_Cylinder_008)) "0, 0, 0" 1.0 1.0 0.0 0 0))
  (Components|MoveComponentTo _drawbridge_cube_006 (Variables|/Script/Engine.SceneComponent|GetRelativeLocation _drawbridge_cube_006) (Math|Rotator|MakeRotator (.roll _relativerotation) -9e+01 (.yaw _relativerotation)) false true 5.0 false)
  (Audio|Components|Audio|Stop _returnvalue_2)
  (Components|DestroyComponent _returnvalue_2)
  (Audio|PlaySoundatLocation "/Game/StarterContent/Audio/Collapse01.Collapse01" _returnvalue "0, 0, 0" 1.0 1.0 0.0 0 0 0 0)
  (Effects|SpawnEmitteratLocation 0 _returnvalue))

(event EventBeginPlay
  (EventDispatchers|BindEventtoOnChargeCompleted (Variables|Default|GetChargeAbleMechanism) (delegate Custom|On%20Activated)))

(fn ConstructionScript)

(fn IsInteracting
  (return false))

(fn HasServerInteraction
  (return false))