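; BP_CharacterAnimTest is a temporary test character that previews weapon and death animations on its mesh.
; It plays animation assets directly, without state logic: looping idle on BeginPlay, one-shot shoot, reload and inspect on input.
; PWHealth's OnDeath triggers the death animation through OnDeathMulti.
; The Map input adds a PW_Map widget on alternate presses, and leftover T-key logic casts the bounty game mode with no further action.
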(event Custom|Server%20Game%20Mode
  ;[1 1 1] Test
  (Utilities|Casting|CastToPW_BountyGameMode_BP (Game|GetGameMode)))

(event Custom|OnDeathEvent
  (params (DamageCauser :type Actor%20Object%20Reference) (DamageCauserController :type Controller%20Object%20Reference))
  ;[1 1 1] DeathAnimationHandling
  (CallFunction|OnDeathMulti))

(event Custom|OnDeathMulti
  ;[1 1 1] DeathAnimationHandling
  (Components|Animation|PlayAnimation (Variables|Character|GetMesh) "/Game/ExternalAssets/SteampunkAndroid2/Animation/Anim_Android2_Death.Anim_Android2_Death" false))

(event Custom|DeathBind
  ;[1 1 1] DeathAnimationHandling
  (EventDispatchers|AssignOnDeath (Variables|Default|GetPW_Health) (delegate Custom|OnDeathEvent)))

(event EventBeginPlay
  (CallFunction|DeathBind)
  (Components|Animation|PlayAnimation (Variables|Character|GetMesh) "/Game/Project_West/Temp/NP/Weapon_Animations/Idle_Anim/A_CharWeaponIdle.A_CharWeaponIdle" true))

(event Input|ActionEvents|InputActionMap
  (params (Key :type Key%20Structure :default "None"))
  ;[1 1 1] Map
  (:Pressed
    (Utilities|FlowControl|FlipFlop
      (:A
        (bind _returnvalue (UserInterface|CreateWidget "/Game/Project_West/Game/Map/PW_Map.PW_Map_C"))
        (UserInterface|Viewport|AddtoViewport _returnvalue 0)))))

(event Input|KeyboardEvents|T
  (params (Key :type Key%20Structure :default "None"))
  ;[1 1 1] Test
  (:Pressed
    (if (Ability|HasAuthority)
      (Utilities|Casting|CastToPW_BountyGameMode_BP (Game|GetGameMode))
      (else
        (CallFunction|ServerGameMode)))))

(event Input|MouseEvents|LeftMouseButton
  (params (Key :type Key%20Structure :default "None"))
  (:Pressed
    (Components|Animation|PlayAnimation (Variables|Character|GetMesh) "/Game/Project_West/Temp/NP/Weapon_Animations/Shooting_Anim/A_CharShooting.A_CharShooting" false)))

(event Input|KeyboardEvents|R
  (params (Key :type Key%20Structure :default "None"))
  (:Pressed
    (Components|Animation|PlayAnimation (Variables|Character|GetMesh) "/Game/Project_West/Temp/NP/Weapon_Animations/Reload_Anim/A_WeaponReload.A_WeaponReload" false)))

(event Input|KeyboardEvents|T
  (params (Key :type Key%20Structure :default "None"))
  (:Pressed
    (Components|Animation|PlayAnimation (Variables|Character|GetMesh) "/Game/Project_West/Temp/NP/Weapon_Animations/Inspect_Anim/A_WeaponInspect.A_WeaponInspect" false)))

(fn ConstructionScript)