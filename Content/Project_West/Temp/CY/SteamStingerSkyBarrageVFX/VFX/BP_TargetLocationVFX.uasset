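; Target location marker actor for the Steam Stinger Sky Barrage VFX, built from static mesh components.
; The construction script pushes the Opacity variable into the Opacity material parameter on two meshes.
; Tick yaws the scene root by a fixed step each frame, so spin speed follows frame rate.
; Tick's scalar parameter write names no parameter, and the decal and dynamic material setup nodes are disconnected.
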(event EventBeginPlay)

(event Collision|EventActorBeginOverlap
  (params (OtherActor :type Actor%20Object%20Reference)))

(event EventTick
  (params (DeltaSeconds :type Float%20%28single-precision%29))
  (Transformation|AddLocalRotation (Variables|Default|GetDefaultSceneRoot) (Math|Rotator|MakeRotator 0.0 0.0 1.0) false false)
  (Rendering|Material|SetScalarParameterValue 0 "None" 0.0 :!class /Script/Engine.KismetMaterialLibrary))

(fn ConstructionScript
  (Utilities|FlowControl|Sequence
    (:then_0
      (Rendering|Material|SetScalarParameterValueonMaterials (Variables|Default|GetStaticMesh) "Opacity" (Variables|Default|GetOpacity)))
    (:then_1
      (Rendering|Material|SetScalarParameterValueonMaterials (Variables|Default|GetStaticMesh1) "Opacity" (Variables|Default|GetOpacity)))))