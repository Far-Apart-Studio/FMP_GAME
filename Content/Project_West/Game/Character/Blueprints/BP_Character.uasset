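; BP_Character is the networked player character, handling crouch, damage feedback, death, overhead names and local UI (hitmarker, pause menu, map).
; Health and damage delegates drive death animation, blood effects and hit sounds.
; Server-to-multicast events relay selected weapon, aim pitch and hit sound, while Tick runs an overhead-name visibility pass over all characters.
; Releasing crouch starts a looping timer that stands up once an upward trace is clear.
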(event OnDeathGlobal(PW_Health)
  (params (OwnerActor :type Actor%20Object%20Reference) (DamageCauser :type Actor%20Object%20Reference) (DamageCauserController :type Controller%20Object%20Reference))
  (Development|PrintString "Trigger"))

(event Custom|Server%20Game%20Mode
  ;[1 1 1] Test
  (Utilities|Casting|CastToPW_BountyGameMode_BP (Game|GetGameMode)))

(event Custom|OnDeathEvent
  (params (OwnerActor :type Actor%20Object%20Reference) (DamageCauser :type Actor%20Object%20Reference) (DamageCauserController :type Controller%20Object%20Reference))
  ;[1 1 1] DeathAnimationHandling
  (CallFunction|OnDeathMulti))

(event Custom|MultiHitSound
  ;[1 1 1] DamageTaken
  (Audio|PlaySound2D "/Game/Project_West/Assets/Audio/SFX/Character/Hit/MeleeHit.MeleeHit" 1.0 1.0 0.0 0 0))

(event Custom|Network%20Rotation
  ;[1 1 1] Networking Player Rotation
  (CallFunction|ROSSetPitch (.pitch (Pawn|GetControlRotation :!class /Script/Engine.Pawn))))

(event Custom|BloodLight
  ;[1 1 1] DamageTaken
  (Niagara|SpawnSystemAttached "/Game/ExternalAssets/YI_BloodDroplets/Particles/CPU/FX_EntranceWound_Shotgun_CPU.FX_EntranceWound_Shotgun_CPU" (Variables|Default|GetBloodLocation) "None" "0, 0, 0" "0, 0, 0" "KeepRelativeOffset" true))

(event Custom|Handle%20OverHead%20Visibility
  (Networking|SwitchHasAuthority
    (:Authority
      (CallFunction|ServerOverHeadVisibility))
    (:Remote
      (CallFunction|ToggleCharacterNames))))

(event Custom|BloodHeavy
  ;[1 1 1] DamageTaken
  (Niagara|SpawnSystemAttached "/Game/ExternalAssets/YI_BloodDroplets/Particles/CPU/FX_AorticSpurt_CPU.FX_AorticSpurt_CPU" (Variables|Default|GetBloodLocation) "None" "0, 0, 0" "0, 0, 0" "KeepRelativeOffset" true))

(event Custom|Server%20OverHead%20Visibility
  (CallFunction|ToggleCharacterNames))

(event Custom|SelectedWeaponServer
  (params (SelectedWeapon :type Integer))
  (CallFunction|SelectedWeaponMulticast SelectedWeapon))

(event Custom|SelectedWeaponMulticast
  (params (SelectedWeapon :type Integer))
  (Variables|Default|SetCurrentSelectedWeapon SelectedWeapon))

(event Custom|SelectedWeapon
  (params (SelectedWeapon :type Integer))
  (CallFunction|SelectedWeaponServer SelectedWeapon))

(event Custom|DamageBind
  ;[1 1 1] DamageTaken
  (EventDispatchers|BindEventtoOnTakeAnyDamage (delegate Custom|TakeDamage)))

(event Custom|OnDeathMulti
  ;[1 1 1] DeathAnimationHandling
  (Components|Animation|PlayAnimation (Variables|Character|GetMesh) "/Game/ExternalAssets/SteampunkAndroid2/Animation/Anim_Android2_Death.Anim_Android2_Death" false)
  (Class|AIPerceptionStimuliSourceComponent|UnregisterfromPerceptionSystem (Variables|Default|GetAIPerceptionStimuliSource)))

(event Custom|DeathBind
  ;[1 1 1] DeathAnimationHandling
  (EventDispatchers|AssignOnDeathGlobal (Variables|Default|GetPW_Health) (delegate Custom|OnDeathEvent)))

(event Custom|TakeDamage
  (params (DamagedActor :type Actor%20Object%20Reference) (Damage :type Float%20%28single-precision%29) (DamageType :type Damage%20Type%20Object%20Reference) (InstigatedBy :type Controller%20Object%20Reference) (DamageCauser :type Actor%20Object%20Reference))
  ;[1 1 1] DamageTaken
  (CallFunction|BloodLight)
  (if (> Damage 5.0)
    (Audio|PlaySound2D 0 1.0 1.0 0.0 0 0)
    (CallFunction|ServerHitSound)
    (if (> Damage 3e+01)
      (CallFunction|BloodHeavy))))

(event Custom|Flip
  (bind _returnvalue (Game|GetPlayerController 0))
  ;[1 1 1] PauseMenu
  (if (not (Variables|Default|GetInteracting))
    (Utilities|FlowControl|FlipFlop
      (:A
        (bind _returnvalue_2 (UserInterface|CreateWidget "/Game/Project_West/Temp/NP/UI/WB_PauseMenu.WB_PauseMenu_C" _returnvalue))
        (UserInterface|Viewport|AddtoViewport _returnvalue_2 0)
        (Input|SetInputModeGameandUI _returnvalue _returnvalue_2 "DoNotLock" true false)
        (Variables|/Script/Engine.PlayerController|SetbShowMouseCursor _returnvalue true))
      (:B
        (Widget|RemovefromParent _returnvalue_2)
        (Input|SetInputModeGameOnly _returnvalue false)
        (Variables|/Script/Engine.PlayerController|SetbShowMouseCursor _returnvalue false)))))

(event Custom|ROS_SetPitch
  (params (Pitch :type Float%20%28double-precision%29))
  ;[1 1 1] Networking Player Rotation
  (CallFunction|MCSetPitch Pitch))

(event Custom|MC_SetPitch
  (params (Pitch :type Float%20%28double-precision%29))
  ;[1 1 1] Networking Player Rotation
  (Variables|Default|SetPitch Pitch))

(event Custom|ServerHitSound
  ;[1 1 1] DamageTaken
  (CallFunction|MultiHitSound))

(event EventBeginPlay
  ;[1 1 1] Begin Play
  (CallFunction|DeathBind)
  (CallFunction|DamageBind)
  (EventDispatchers|BindEventtoOnCameraRotationChange (EventDispatchers|CreateEvent :!event Custom|Network%20Rotation))
  (Utilities|FlowControl|Delay 2.0)
  (bind _aswb_overhead_ui (Utilities|Casting|CastToWB_OverheadUI (UserInterface|GetWidget (Variables|Default|GetOverhead%20Widget))))
  (Variables|Default|SetOverheadRef _aswb_overhead_ui)
  (CallFunction|LoadOverHeadName)
  (bind _aspw_player_controller_bp (Utilities|Casting|CastToPW_PlayerController_BP (Pawn|GetController)))
  (EventDispatchers|AssignOnNameChanged _aspw_player_controller_bp (EventDispatchers|CreateEvent :!event SetOverheadName))
  (CallFunction|MakeHitmarker))

(event EventTick
  (params (DeltaSeconds :type Float%20%28single-precision%29))
  (CallFunction|HandleOverHeadVisibility))

(event EventStopCrouching
  (bind _springarm (Variables|Default|GetSpringArm))
  (bind _returnvalue (Transformation|GetWorldLocation _springarm))
  ;[1 1 1] Crouch
  (bind _returnvalue_2 (Collision|LineTraceByChannel _returnvalue (+ _returnvalue (* (Math|Vector|GetUpVector _springarm) 1e+02)) "TraceTypeQuery1" false 0 "None" true "(R=1.000000,G=0.000000,B=0.000000,A=1.000000)" "(R=0.000000,G=1.000000,B=0.000000,A=1.000000)" 0.1))
  (if (not _returnvalue_2)
    (Utilities|Time|ClearandInvalidateTimerbyHandle (stale Input|ActionEvents|InputActionCrouch _returnvalue))
    (Character|UnCrouch)))

(event Input|ActionEvents|InputActionMap
  (params (Key :type Key%20Structure :default "None"))
  ;[1 1 1] Map
  (:Pressed
    (Utilities|FlowControl|FlipFlop
      (:A
        (bind _returnvalue (UserInterface|CreateWidget "/Game/Project_West/Game/Map/PW_Map.PW_Map_C"))
        (UserInterface|Viewport|AddtoViewport _returnvalue 0))
      (:B
        (Widget|RemovefromParent _returnvalue)))))

(event Input|ActionEvents|InputActionCrouch
  (params (Key :type Key%20Structure :default "None"))
  ;[1 1 1] Crouch
  (:Pressed
    (if (AI|Components|NavMovement|IsMovingonGround (Variables|Character|GetCharacterMovement))
      (Character|Crouch)))
  (:Released
    (if (AI|Components|NavMovement|IsCrouching (Variables|Character|GetCharacterMovement))
      (bind _returnvalue (Utilities|Time|SetTimerbyEvent (delegate EventStopCrouching) 0.01 true)))))

(event Input|ActionEvents|InputActionReturn
  (params (Key :type Key%20Structure :default "None"))
  (bind _returnvalue (Game|GetPlayerController 0))
  ;[1 1 1] PauseMenu
  (:Pressed
    (if (not (Variables|Default|GetInteracting))
      (Utilities|FlowControl|FlipFlop
        (:A
          (bind _returnvalue_2 (UserInterface|CreateWidget "/Game/Project_West/Temp/NP/UI/WB_PauseMenu.WB_PauseMenu_C" _returnvalue))
          (UserInterface|Viewport|AddtoViewport _returnvalue_2 0)
          (Input|SetInputModeGameandUI _returnvalue _returnvalue_2 "DoNotLock" true false)
          (Variables|/Script/Engine.PlayerController|SetbShowMouseCursor _returnvalue true))
        (:B
          (Widget|RemovefromParent _returnvalue_2)
          (Input|SetInputModeGameOnly _returnvalue false)
          (Variables|/Script/Engine.PlayerController|SetbShowMouseCursor _returnvalue false))))))

(event Input|KeyboardEvents|T
  (params (Key :type Key%20Structure :default "None"))
  ;[1 1 1] Test
  (:Pressed
    (if (Ability|HasAuthority)
      (Utilities|Casting|CastToPW_BountyGameMode_BP (Game|GetGameMode))
      (else
        (CallFunction|ServerGameMode)))))

(fn ConstructionScript
  (Class|PWCharacter|SetWidgetComponent (Variables|Default|GetOverhead%20Widget))
  (Class|PWCharacter|SetItemHolderComponent (Variables|Default|GetItem%20Holder))
  (Class|PWCharacter|SetSpringArmComponent (Variables|Default|GetSpringArm))
  (Class|PWCharacter|SetCameraComponent (Variables|Default|GetCamera)))

(fn SetOverheadName
  (params (name :type String))
  (bind _aswb_overhead_ui (Utilities|Casting|CastToWB_OverheadUI (UserInterface|GetWidget (Variables|Default|Get_overheadWidget))))
  (Default|SetName _aswb_overhead_ui name)
  (Development|PrintString (Utilities|String|Append "Name : " name)))

(fn LoadOverHeadName
  (bind _aswb_overhead_ui (Utilities|Casting|CastToWB_OverheadUI (UserInterface|GetWidget (Variables|Default|Get_overheadWidget))))
  (Default|SetName _aswb_overhead_ui (Variables|Default|Get_playerName)))

(fn ToggleNameVisibility
  (params (visibility :type Boolean))
  (bind _overheadref (Variables|Default|GetOverheadRef))
  (Utilities|IsValid _overheadref
    (:Is%20Valid
      (Default|Opacity _overheadref))))

(fn ToggleCharacterNames
  (bind _namevisilitydistance (Variables|Default|GetNameVisilityDistance))
  (bind _outactors (Actor|GetAllActorsOfClass "BP_Character_C"))
  (for _array_element _outactors
    (if (< (Transformation|GetDistanceTo _array_element self) _namevisilitydistance)
      (Variables|Default|SetOpacityDistance 1.0)
      (else
        (Variables|Default|SetOpacityDistance (Math|Float|Clamp(Float) (- 1.0 (/ (- (Transformation|GetDistanceTo _array_element self) _namevisilitydistance) 5e+02))))))
    (CallFunction|ToggleNameVisibility _array_element false)))

(fn SelectedWeaponID
  (params (WeaponID :type Integer))
  (Variables|Default|SetCurrentSelectedWeapon WeaponID))

(fn ActivateHitmarker
  (bind _hitmarkerref (Variables|Default|GetHitmarkerRef))
  (Utilities|IsValid _hitmarkerref
    (:Is%20Valid
      (Default|ActivateHitmark _hitmarkerref))))

(fn MakeHitmarker
  (bind _returnvalue (UserInterface|CreateWidget "/Game/Project_West/Temp/TB/Hitmarker.Hitmarker_C"))
  (UserInterface|Viewport|AddtoViewport _returnvalue 0)
  (Variables|Default|SetHitmarkerRef _returnvalue))