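; Player controller component that shows the session's side objectives on screen and reacts when their state changes.
; StartUp creates the WB_SessionTasks widget for the owning PW_PlayerController_BP, then adds a task widget for each active objective in the supplied manager.
; A delegate bound on that widget passes state changes to the controller's BP_NotificationHandler and, only if that exists, removes the objective from BP_CompassLocator.
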(event EventBeginPlay)

(event EventTick
  (params (DeltaSeconds :type Float%20%28single-precision%29)))

(fn GetControllerandCreateWidget
  (bind _aspw_player_controller_bp (Utilities|Casting|CastToPW_PlayerController_BP (Components|GetOwner))
    (:then
      (bind _output_get (Variables|Default|SetPlayer%20Controller%20BP _aspw_player_controller_bp))
      (bind _returnvalue (UserInterface|CreateWidget "/Game/Project_West/UI/Objectives/WB_SessionTasks.WB_SessionTasks_C" _output_get))
      (EventDispatchers|BindEventtoOnTaskStateChanged _returnvalue (EventDispatchers|CreateEvent :!event OnTaskStateChanged))
      (bind _output_get_2 (Variables|Default|SetSessionTaskBp _returnvalue))
      (UserInterface|Viewport|AddtoViewport _output_get_2 0))
    (:CastFailed
      (Development|PrintString "Cannot find Controller"))))

(fn TaskManager
  (params (S0%20Manager :type BP%20Side%20Objective%20Manager%20Object%20Reference))
  (bind _output_get (Variables|Default|SetS0%20Manager S0%20Manager))
  (for _array_element (Variables|/Script/PROJECT_WEST.PW_SideObjectiveManager|Get_activeObjectives _output_get)
    (bind _taskwidget (Default|AddTaskWidget (Variables|Default|GetSessionTaskBp)))
    (Default|SetUp _taskwidget _array_element)))

(fn StartUp
  (params (S0%20Manager :type BP%20Side%20Objective%20Manager%20Object%20Reference))
  (CallFunction|GetControllerandCreateWidget)
  (CallFunction|TaskManager S0%20Manager))

(fn OnTaskStateChanged
  (params (notification :type Notification%20Entry%20Structure) (sideObjecive :type PW%20Side%20Objective%20Object%20Reference))
  (bind _player_controller_bp (Variables|Default|GetPlayer%20Controller%20BP))
  (bind _returnvalue (Actor|GetComponentbyClass _player_controller_bp "/Game/Project_West/Game/Compass/BP_CompassLocator.BP_CompassLocator_C"))
  (bind _returnvalue_2 (Actor|GetComponentbyClass _player_controller_bp "/Game/Project_West/Game/NotficationSystem/BP_NotificationHandler.BP_NotificationHandler_C"))
  (Utilities|IsValid _returnvalue_2
    (:Is%20Valid
      (Default|DisplayNotification _returnvalue_2 notification)
      (Utilities|IsValid _returnvalue
        (:Is%20Valid
          (Default|RemoveTaskfromCompass _returnvalue sideObjecive))))))