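; BP_DebtCollector is an interactable debt collector that displays the debt amount and reacts to the player's interaction.
; On BeginPlay it binds to the debt-amount-changed delegate, which pushes each new value as text into the WB_Debt widget hosted by InteractWidget.
; On interaction it plays a payment sound at the world origin and adds a WB_ThankYouNote widget to the viewport, with no debt deduction in this graph.
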(event Custom|_onDebtAmountChanged_Event
  (params (DebtAmount :type Integer))
  ;[1 1 1] Set Debt Value on UI
  (bind _aswb_debt (Utilities|Casting|CastToWB_Debt (UserInterface|GetWidget (Variables|Default|GetInteractWidget))))
  (Default|SetDebtValueText _aswb_debt (Utilities|String|ToString(Integer) DebtAmount)))

(event EventBeginPlay
  ;[1 1 1] Set Debt Value on UI
  (EventDispatchers|AssignOnDebtAmountChanged (delegate Custom|_onDebtAmountChanged_Event)))

(event EventOnInteracted
  (params (status :type Boolean))
  (Audio|PlaySoundatLocation "/Game/Project_West/Assets/Audio/SFX/Misc/SW_PayDebtCollector.SW_PayDebtCollector" "0, 0, 0" "0, 0, 0" 1.0 1.0 0.0 0 0 0 0)
  (bind _returnvalue (UserInterface|CreateWidget "/Game/Project_West/UI/Misc/WB_ThankYouNote.WB_ThankYouNote_C"))
  (UserInterface|Viewport|AddtoViewport _returnvalue 0))

(fn ConstructionScript)