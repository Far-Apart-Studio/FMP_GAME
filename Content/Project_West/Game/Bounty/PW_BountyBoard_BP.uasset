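; Lobby bounty board actor that shows bounties on a widget and lets players vote on which one to play.
; The authority populates the bounty list, button presses send votes through the player controller, and vote delegates refresh counts and button locking.
; The authority enables Start once votes cover all session players; pressing it activates the lobby game mode's transition portal.
; A successful vote also grants the player a hard-coded money reward.
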(event Custom|BountyDataListChanged_Event
  (params (bountyDataList :type Array%20of%20Bounty%20Data%20Entry%20Structures))
  (CallFunction|SetBountyInfo bountyDataList))

(event Custom|OnBoardOpened_Event)

(event Custom|OnBoardClosed_Event)

(event EventBeginPlay
  (CallFunction|SetUpBountyWidgetButtons)
  (EventDispatchers|AssignOnBoardOpened (delegate Custom|OnBoardOpened_Event))
  (EventDispatchers|AssignOnBoardClosed (delegate Custom|OnBoardClosed_Event))
  (EventDispatchers|AssignBountyDataListChanged (delegate Custom|BountyDataListChanged_Event))
  (EventDispatchers|BindEventtoBountyVoteDataChanged (EventDispatchers|CreateEvent :!event OnVoteChanged))
  (bind _playercontroller (CallFunction|GetPlayerController))
  (EventDispatchers|AssignVoteChangedDelegate _playercontroller (EventDispatchers|CreateEvent :!event OnVoteStatusChanged))
  (if (Ability|HasAuthority)
    (Class|PWBountyBoard|PopulateBountyDataList)
    (else
      (CallFunction|SetBountyInfo (Variables|Default|Get_bountyDataList))))
  (Default|ToggleStartButton (Variables|Default|GetBounty%20Widget) false))

(event Collision|EventActorBeginOverlap
  (params (OtherActor :type Actor%20Object%20Reference)))

(event EventTick
  (params (DeltaSeconds :type Float%20%28single-precision%29)))

(fn ConstructionScript)

(fn SetBountyInfo
  (params (BountyDatas :type Array%20of%20Bounty%20Data%20Entry%20Structures))
  (bind _aspw_bounty_wbp (Utilities|Casting|CastToPW_Bounty_WBP (UserInterface|GetWidget (Variables|Default|Get_bountyBoardWidget))))
  (Default|SetBountyInfoList _aspw_bounty_wbp BountyDatas))

(fn SetUpBountyWidgetButtons
  (bind _aspw_bounty_wbp (Utilities|Casting|CastToPW_Bounty_WBP (UserInterface|GetWidget (Variables|Default|Get_bountyBoardWidget))))
  (Variables|Default|SetBounty%20Widget _aspw_bounty_wbp)
  (Default|GetBountySectionButtons _aspw_bounty_wbp)
  (EventDispatchers|BindEventtoBountyButtonPressed _aspw_bounty_wbp (EventDispatchers|CreateEvent :!event OnBountyButtonPressed))
  (EventDispatchers|BindEventtoOnStartPressed _aspw_bounty_wbp (EventDispatchers|CreateEvent :!event OnStartButtonPressed)))

(fn OnBountyButtonPressed
  (params (BountyButton :type Bounty%20Selection%20Object%20Reference))
  (bind _playercontroller (CallFunction|GetPlayerController))
  (Utilities|IsValid _playercontroller
    (:Is%20Valid
      (Class|PWPlayerController|DoVotetoBounty _playercontroller (.index (Utilities|Struct|BreakBountyDataEntry (Variables|/Game/Project_West/UI/Bounty/Widget_Blueprints/BountySelection.BountySelection_C|GetBountyData BountyButton)))))))

(fn EnableTransitionPortal
  (bind _aspw_lobby_game_mode_bp (Utilities|Casting|CastToPW_LobbyGameMode_BP (Game|GetGameMode)))
  (Class|PWTransitionPortal|ToggleActivation (Variables|/Script/PROJECT_WEST.PW_LobbyGameMode|Get_transitionPortal _aspw_lobby_game_mode_bp) true)
  (Default|ToggleButtonsInteractivity (Variables|Default|GetBounty%20Widget) false -1))

(fn GetPlayerController
  (bind _playercontroller (Variables|Default|GetPlayerController))
  (Utilities|IsValid _playercontroller
    (:Is%20Valid
      (return _playercontroller))
    (:Is%20Not%20Valid
      (bind _aspw_game_state (Utilities|Casting|CastToPW_GameState (Game|GetGameState)))
      (bind _returnvalue (Class|PWGameState|GetLocalPlayerController _aspw_game_state))
      (return _returnvalue))))

(fn OnVoteChanged
  (params (bountyVoteData :type Bounty%20Vote%20Data%20Structure%20%28by%20ref%29))
  (for (_array_element _array_index) (Utilities|Struct|BreakBountyVoteData bountyVoteData)
    (Default|SetVotes (Utilities|Array|Get(acopy) (Variables|/Game/Project_West/UI/Bounty/Widget_Blueprints/PW_Bounty_WBP.PW_Bounty_WBP_C|GetBounty%20Selection%20List (Variables|Default|GetBounty%20Widget)) _array_index) (Utilities|Struct|BreakBountyVoteDataEntry _array_element)))
  (CallFunction|TryEnableStartButton)
  (return))

(fn OnStartButtonPressed
  (Variables|Default|Set_isActivated false)
  (CallFunction|EnableTransitionPortal))

(fn TryEnableStartButton
  (Networking|SwitchHasAuthority
    (:Authority
      (bind _aspw_lobby_game_mode_bp (Utilities|Casting|CastToPW_LobbyGameMode_BP (Game|GetGameMode)))
      (bind _returnvalue (Class|PWBountyBoard|GetTotalVotes))
      (Default|ToggleStartButton (Variables|Default|GetBounty%20Widget) (>= _returnvalue (Class|PWGameMode|GetNumPlayerinSession _aspw_lobby_game_mode_bp))))))

(fn OnVoteStatusChanged
  (params (bsuccess :type Boolean) (bountyIndex :type Integer))
  (if bsuccess
    (Default|ToggleButtonsInteractivity (Variables|Default|GetBounty%20Widget) false bountyIndex)
    (bind _playercontroller (CallFunction|GetPlayerController))
    (Class|PWPlayerController|AddMoney _playercontroller 50000)
    (else
      (Default|ToggleButtonsInteractivity (Variables|Default|GetBounty%20Widget) true -1))))