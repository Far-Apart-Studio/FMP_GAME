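; BP_NotificationHandler is a component owned by the player controller that drives the on-screen notification and interaction prompt HUD.
; SetUp caches the controller and its character, creates the WB_NotificationHud widget, and binds to the controller's notification event and the character's interaction trace.
; Notification entries are forwarded to the widget.
; Traced actors show their BP_InteractionPrompt, which hides when the actor or that component is missing.
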(event EventBeginPlay)

(fn SetPlayerController
  (bind _asbp_player_controller (Utilities|Casting|CastToBP_PlayerController (Components|GetOwner))
    (:then
      (bind _output_get (Variables|Default|SetPlayer%20Controller%20BP _asbp_player_controller))
      (EventDispatchers|BindEventtoOnNotificationTriggered _output_get (EventDispatchers|CreateEvent :!event DisplayNotification))
      (bind _asbp_character (Utilities|Casting|CastToBP_Character (Pawn|GetControlledPawn _output_get)))
      (Variables|Default|SetBP%20Character _asbp_character))
    (:CastFailed
      (Development|PrintString "BP_Cast Failed" true true "(R=0.000000,G=0.660000,B=1.000000,A=1.000000)" 5.0))))

(fn CreateNotgificationHUD
  (bind _returnvalue (UserInterface|CreateWidget "/Game/Project_West/UI/Notification/WB_NotificationHud.WB_NotificationHud_C"))
  (bind _output_get (Variables|Default|SetNotificationHUD _returnvalue))
  (UserInterface|Viewport|AddtoViewport _output_get 0))

(fn SetUp
  (CallFunction|SetPlayerController)
  (CallFunction|CreateNotgificationHUD)
  (CallFunction|SetUpInteractionPrompt))

(fn DisplayNotification
  (params (notificationEntry :type Notification%20Entry%20Structure))
  (Default|AddNotification (Variables|Default|GetNotificationHUD) notificationEntry))

(fn SetUpInteractionPrompt
  (EventDispatchers|BindEventtoOnTraceInteractable (Actor|GetComponentbyClass (Variables|Default|GetBP%20Character) "/Script/PROJECT_WEST.PW_InteractionComponent") (EventDispatchers|CreateEvent :!event OnInteratableTrace)))

(fn OnInteratableTrace
  (params (interactedActor :type Actor%20Object%20Reference))
  (bind _returnvalue (Actor|GetComponentbyClass interactedActor "/Game/Project_West/Game/Interaction/BP_InteractionPrompt.BP_InteractionPrompt_C"))
  (Utilities|IsValid interactedActor
    (:Is%20Valid
      (Utilities|IsValid _returnvalue
        (:Is%20Valid
          (Default|DisplayInteractionPrompt (Variables|Default|GetNotificationHUD) _returnvalue))
        (:Is%20Not%20Valid
          (Default|HideInteractionPrompt (Variables|Default|GetNotificationHUD) :!label _label))))
    (:Is%20Not%20Valid
      (goto _label))))

(fn ToggleVisibility
  (Widget|SetVisibility (Variables|Default|GetNotificationHUD) "Visible"))