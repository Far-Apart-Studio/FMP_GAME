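; Weapon Blueprint for Project_West that adds sound, visual effects and prototype recoil to weapon events.
; BeginPlay caches effects from WeaponVisualData and binds handlers to fire, stop-fire, hit and reload delegates.
; Firing routes through Server to Multi for muzzle flash, sound and a revolver montage; hits spawn Niagara beam tracers sized by horizontal distance.
; Temporary timeline recoil drives owner pitch and yaw, reversing when firing stops.
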(event Custom|Reload
  (Audio|SpawnSoundAttached (Variables|Default|GetWeaponReloadSound) (Variables|Default|Get_muzzleLocation) "None" "0, 0, 0" "0, 0, 0" "KeepRelativeOffset" false 0.5 1.0 0.0 0 0))

(event Custom|Server
  ;[1 1 1] FIRE EVENT (EXAMPLE OF HOW TODO THE SOUND AND VISUALS FOR WEAPON)
  (CallFunction|Multi))

(event Custom|OnFireStopRecoil
  ;[1 1 1] Prototype Recoil / Testing Timeline Recoil / NOT BEING KEPT
  (bind (_direction _pitch _yaw) (Timeline|Recoil%20Timeline Reverse)
    (:Update
      (switch Utilities|FlowControl|Switch|SwitchonETimelineDirection _direction
        (:Forward
          (CallFunction|ModifyYawPitch _pitch _yaw))
        (:Backward
          (CallFunction|ModifyYawPitch (* _pitch -1.0) (* _yaw -1.0)))))))

(event Custom|Multi
  (bind __muzzlelocation (Variables|Default|Get_muzzleLocation))
  ;[1 1 1] FIRE EVENT (EXAMPLE OF HOW TODO THE SOUND AND VISUALS FOR WEAPON)
  (Audio|SpawnSoundAttached (Variables|Default|GetWeaponShootSound) __muzzlelocation "None" "0, 0, 0" "0, 0, 0" "KeepRelativeOffset" false 0.5 1.0 0.0 0 0)
  (Effects|SpawnEmitterAttached (Variables|Default|GetWeaponMuzzleFlash) __muzzlelocation "None" "0, 0, 0" "0, 0, 0" "0.100000,0.100000,0.100000")
  (bind _asbp_character (Utilities|Casting|CastToBP_Character (Components|GetOwner)))
  (Animation|PlayAnimMontage _asbp_character "/Game/Project_West/Assets/Animations/Character_Animations/Revolver_Animations/Shooting_Anim/AM_RevolverShoot.AM_RevolverShoot" 0.7 "None"))

(event Custom|OnHit
  (params (HitResult :type Hit%20Result%20Structure) (StartPoint :type Vector) (EndPoint :type Vector))
  ;[1 1 1] Bullet Tracer VFX
  (bind _returnvalue (Niagara|SpawnSystematLocation "/Game/Project_West/Assets/Art/VFX/BulletTracer/FXS_BulletTracerBeam.FXS_BulletTracerBeam" StartPoint (Transformation|GetActorRotation)))
  (Niagara|SetNiagaraVariable(Float) _returnvalue "BeamLength" (Math|Vector|VectorLengthXY (- StartPoint EndPoint))))

(event Custom|OnFire
  ;[1 1 1] FIRE EVENT (EXAMPLE OF HOW TODO THE SOUND AND VISUALS FOR WEAPON)
  (CallFunction|Server))

(event Custom|OnFireRecoil
  ;[1 1 1] Prototype Recoil / Testing Timeline Recoil / NOT BEING KEPT
  (bind (_direction _pitch _yaw) (Timeline|Recoil%20Timeline Play)
    (:Update
      (switch Utilities|FlowControl|Switch|SwitchonETimelineDirection _direction
        (:Forward
          (CallFunction|ModifyYawPitch _pitch _yaw))
        (:Backward
          (CallFunction|ModifyYawPitch (* _pitch -1.0) (* _yaw -1.0)))))))

(event EventBeginPlay
  (Variables|Default|SetWeaponShootSound (Variables|/Script/PROJECT_WEST.PW_WeaponVisualData|Get_fireSound (Variables|Default|Get_weaponVisualData)))
  (Variables|Default|SetWeaponMuzzleFlash (Variables|/Script/PROJECT_WEST.PW_WeaponVisualData|Get_muzzleFlash (Variables|Default|Get_weaponVisualData)))
  (Variables|Default|SetWeaponReloadSound (Variables|/Script/PROJECT_WEST.PW_WeaponVisualData|Get_reloadSound (Variables|Default|Get_weaponVisualData)))
  (EventDispatchers|AssignOnWeaponFireDelegate (EventDispatchers|CreateEvent :!event Custom|OnFire))
  (EventDispatchers|BindEventtoOnWeaponHit (EventDispatchers|CreateEvent :!event Custom|OnHit))
  (EventDispatchers|BindEventtoOnWeaponFireDelegate (EventDispatchers|CreateEvent :!event Custom|OnFireRecoil))
  (EventDispatchers|AssignOnWeaponStopFire (EventDispatchers|CreateEvent :!event Custom|OnFireStopRecoil))
  (EventDispatchers|BindEventtoOnWeaponBeginReload (EventDispatchers|CreateEvent :!event Custom|Reload)))

(fn ConstructionScript)

(fn ModifyYawPitch
  (params (Pitch :type Float%20%28single-precision%29) (Yaw :type Float%20%28single-precision%29))
  (bind _aspw_character (Utilities|Casting|CastToPW_Character (Components|GetOwner)))
  (Pawn|Input|AddControllerPitchInput _aspw_character Pitch)
  (Pawn|Input|AddControllerYawInput _aspw_character Yaw))