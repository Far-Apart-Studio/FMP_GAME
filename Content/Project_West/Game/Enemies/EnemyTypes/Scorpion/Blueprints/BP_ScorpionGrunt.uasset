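; Scorpion grunt enemy with melee and ranged attacks against player characters.
; Melee moves to the AI controller's target, plays a random montage and damages characters overlapping the hitbox.
; The shot checks line of sight, halts and charges, locks aim just before a hitscan beam fires, and disables stagger meanwhile.
; Separate functions randomly launch a projectile and map movement states to walk speeds.
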(event Custom|AttackServerM
  ;[1 1 1] Melee Attack
  (Animation|Montage|PlayMontage (Variables|Character|GetMesh) (.OutItem (Utilities|Array|Random (Variables|Default|GetMeleeAttackAnims)))
    (:OnCompleted
      _)
    (:OnInterrupted
      _))
  (Default|CallOnAttackEnd))

(event Custom|AttackAnimation
  ;[1 1 1] Melee Attack
  (CallFunction|AttackServerM))

(event Custom|ShootAttackMulti
  (params (Player :type Actor%20Object%20Reference))
  (bind _returnvalue (Transformation|GetActorLocation))
  (bind _scene (Variables|Default|GetScene))
  ;[1 1 1] ShootAttack
  (Components|Movement|StopMovementImmediately (Variables|Character|GetCharacterMovement))
  (Variables|Default|SetCanBeStaggered false)
  (Variables|Default|SetTargeted%20Player Player)
  (Variables|/Script/Engine.CharacterMovementComponent|SetMaxWalkSpeed (Variables|Character|GetCharacterMovement) 0.0)
  (bind _outhit (Collision|LineTraceByChannel (Transformation|GetActorLocation) (Transformation|GetActorLocation (Variables|Default|GetTargeted%20Player)) "TraceTypeQuery1" false 0 "None"))
  (if (== (.HitActor (Collision|BreakHitResult _outhit)) (Variables|Default|GetTargeted%20Player))
    (Audio|PlaySoundatLocation "/Game/Project_West/Temp/TB/ChargeSound.ChargeSound" (Transformation|GetActorLocation) "0, 0, 0" 1.0 1.0 0.0 0 0 0 0)
    (Niagara|SpawnSystematLocation "/Game/Project_West/Assets/Art/VFX/Rifle/RifleImpact/FXS_RifleImpact.FXS_RifleImpact" (Transformation|GetWorldLocation (Variables|Default|GetScene)))
    (Utilities|FlowControl|Delay 1.0)
    (CallFunction|ClearFocus)
    (Variables|Default|SetActorLocation (Transformation|GetActorLocation (Variables|Default|GetTargeted%20Player)))
    (Utilities|FlowControl|Delay 0.03)
    (if (> (Variables|/Script/PROJECT_WEST.PW_HealthComponent|Get_currentHealth (Variables|Default|GetPW_Health)) 0.0)
      (bind _outhit_2 (Collision|LineTraceByChannel (Transformation|GetWorldLocation (Variables|Default|GetScene)) (+ _returnvalue (* (Math|Vector|GetForwardVector (Math|Rotator|FindLookatRotation _returnvalue (Variables|Default|GetActorLocation))) 1e+04)) "TraceTypeQuery1" false 0 "None"))
      (Animation|Montage|PlayMontage (Variables|Character|GetMesh) "/Game/Project_West/Game/Enemies/EnemyTypes/Scorpion/Animation/AM_ScorpionShootAttack.AM_ScorpionShootAttack"
        (:then
          (bind _returnvalue_2 (Niagara|SpawnSystematLocation "/Game/Project_West/Assets/Art/VFX/Rifle/RifleTracer/FXS_BulletTracerBeamRifle.FXS_BulletTracerBeamRifle" (Transformation|GetWorldLocation _scene) (Transformation|GetWorldRotation _scene)))
          (Effects|Components|ParticleSystem|SetVectorParameter _returnvalue_2 "BeamStart" (Transformation|GetWorldLocation (Variables|Default|GetScene)))
          (if (.bBlockingHit (Collision|BreakHitResult _outhit_2))
            (Effects|Components|ParticleSystem|SetVectorParameter _returnvalue_2 "BeamEnd" (.ImpactPoint (Collision|BreakHitResult _outhit_2)))
            (else
              (Effects|Components|ParticleSystem|SetVectorParameter _returnvalue_2 "BeamEnd" (.TraceEnd (Collision|BreakHitResult _outhit_2)))))
          (Audio|PlaySoundatLocation "/Game/StarterContent/Audio/Explosion_Cue.Explosion_Cue" (Transformation|GetActorLocation) "0, 0, 0" 1.0 1.0 0.0 0 0 0 0)
          (bind _asbp_character (Utilities|Casting|CastToBP_Character (.HitActor (Collision|BreakHitResult _outhit_2)))
            (:then
              (Game|Damage|ApplyDamage _asbp_character (Variables|Default|GetShootDamageAmount) 0 self)
              (Variables|Default|SetCanBeStaggered true))
            (:CastFailed
              (Variables|Default|SetCanBeStaggered true))))
        (:OnCompleted
          (Default|CallOnAttackEnd))))
    (else
      (Variables|Default|SetCanBeStaggered true)
      (Default|CallOnAttackEnd))))

(event Custom|ClearFocus
  ;[1 1 1] ShootAttack
  (if (Ability|HasAuthority)
    (AI|ClearFocus (Variables|Default|GetBP%20Base%20AIController))))

(event EventBeginPlay
  (|CallParentFunction) ; This node is disabled and will not be called.\nDrag off pins to build functionality.
)

(event Collision|EventActorBeginOverlap
  (params (OtherActor :type Actor%20Object%20Reference)))

(event EventTick
  (params (DeltaSeconds :type Float%20%28single-precision%29))
  (|CallParentFunction DeltaSeconds) ; This node is disabled and will not be called.\nDrag off pins to build functionality.
)

(event EventAttack
  ;[1 1 1] Melee Attack
  (bind _asbp_base_aicontroller (Utilities|Casting|CastToBP_BaseAIController (Pawn|GetController)))
  (Utilities|IsValid (Variables|/Game/Project_West/Game/Enemies/EnemyTypes/Scorpion/Behaviour/ControllerBB/BP_BaseAIController.BP_BaseAIController_C|GetAttack%20Target _asbp_base_aicontroller)
    (:Is%20Valid
      (AI|AIMoveTo self "0, 0, 0" (Variables|/Game/Project_West/Game/Enemies/EnemyTypes/Scorpion/Behaviour/ControllerBB/BP_BaseAIController.BP_BaseAIController_C|GetAttack%20Target _asbp_base_aicontroller) 5.0 false
        (:then
          (Utilities|FlowControl|Delay 0.25)
          (CallFunction|AttackAnimation)
          (Utilities|FlowControl|Delay 0.5)
          (for _array_element (Collision|GetOverlappingActors (Variables|Default|GetPlayerAttackHitbox) "/Game/Project_West/Game/Character/Blueprints/BP_Character.BP_Character_C" :!class /Script/Engine.PrimitiveComponent)
            (if (Collision|IsOverlappingActor (Variables|Default|GetPlayerAttackHitbox) _array_element :!class /Script/Engine.PrimitiveComponent)
              (Game|Damage|ApplyDamage _array_element (Variables|Default|GetMeleeDamageAmount) 0 self))))))
    (:Is%20Not%20Valid
      (Default|SetStatePassive _asbp_base_aicontroller))))

(event EventShootAttack
  (params (TargetedPlayer :type Actor%20Object%20Reference))
  ;[1 1 1] ShootAttack
  (CallFunction|ShootAttackMulti TargetedPlayer))

(fn ConstructionScript
  (|CallParentFunction))

(fn ShootScorpion
  (params (self2 :type Actor%20Object%20Reference))
  (bind _scene (Variables|Default|GetScene))
  (if (not (Variables|Default|GetShootCooldown))
    (if (> (Math|Random|RandomFloatinRange 1.0 4.0) 3.0)
      (Variables|Default|SetShootCooldown true)
      (Game|SpawnActorfromClass "/Game/Project_West/Temp/TB/BP_PrototypeAIProjectile.BP_PrototypeAIProjectile_C" (Math|Transform|MakeTransform (Transformation|GetWorldLocation (Variables|Default|GetScene)) (Math|Rotator|FindLookatRotation (Transformation|GetActorLocation) (Transformation|GetActorLocation (Variables|Default|GetPlayerVar))) "1.000000,1.000000,1.000000") "Undefined" "MultiplyWithRoot" 0 0)
      (Audio|SpawnSoundAttached "/Game/StarterContent/Audio/Explosion_Cue.Explosion_Cue" _scene "None" "0, 0, 0" "0, 0, 0" "KeepRelativeOffset" false 1.0 1.0 0.0 0 0)
      (Effects|SpawnEmitterAttached "/Game/StarterContent/Particles/P_Explosion.P_Explosion" _scene "None" "0, 0, 0" "0, 0, 0" "0.500000,0.500000,0.500000"))))

(fn SetMovementSpeed
  (params (NewParam :type E_MovementSpeed%20Enum :default "NewEnumerator0"))
  (bind _output_get (Variables|/Script/Engine.CharacterMovementComponent|SetMaxWalkSpeed (Variables|Character|GetCharacterMovement) (Utilities|Select :Index NewParam :NewEnumerator0 0.0 :NewEnumerator1 5e+02 :NewEnumerator2 6.5e+02 :NewEnumerator3 8e+02 :NewEnumerator4 2.4e+03)))
  (return _output_get))