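; Mini scorpion enemy that chases and melees players and plays its sound at random intervals until dead.
; Attack starts a move toward the AI controller's target or sets the controller passive if none is valid.
; Without waiting for arrival, timed delays lead into a random montage, then damage to characters overlapping the hitbox.
; Montage completion or interruption signals attack end, and GetIdealRange supplies its attack and defend radii.
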(event Custom|AttackServerM
  ;[1 1 1] MeleeAttack
  (Animation|Montage|PlayMontage (Variables|Character|GetMesh) (.OutItem (Utilities|Array|Random (Variables|Default|GetMeleeAttackAnims)))
    (:OnCompleted
      _)
    (:OnInterrupted
      _))
  (Default|CallOnAttackEnd))

(event Custom|AttackAnimation
  ;[1 1 1] MeleeAttack
  (CallFunction|AttackServerM))

(event EventBeginPlay
  (|CallParentFunction)
  (Audio|PlaySoundatLocation "/Game/Project_West/Temp/TB/MiniScorps.MiniScorps" (Transformation|GetActorLocation) "0, 0, 0" 1.0 1.0 0.0 0 0 0 0 :!label _label)
  (Utilities|FlowControl|Delay (Math|Random|RandomFloatinRange 5.0 15.0))
  (if (not (Variables|Default|GetDead))
    (goto _label)))

(event Collision|EventActorBeginOverlap
  (params (OtherActor :type Actor%20Object%20Reference)))

(event EventTick
  (params (DeltaSeconds :type Float%20%28single-precision%29))
  (|CallParentFunction DeltaSeconds) ; This node is disabled and will not be called.\nDrag off pins to build functionality.
)

(event EventAttack
  ;[1 1 1] MeleeAttack
  (bind _asbp_base_aicontroller (Utilities|Casting|CastToBP_BaseAIController (Pawn|GetController)))
  (Utilities|IsValid (Variables|/Game/Project_West/Game/Enemies/EnemyTypes/Scorpion/Behaviour/ControllerBB/BP_BaseAIController.BP_BaseAIController_C|GetAttack%20Target _asbp_base_aicontroller)
    (:Is%20Valid
      (AI|AIMoveTo self "0, 0, 0" (Variables|/Game/Project_West/Game/Enemies/EnemyTypes/Scorpion/Behaviour/ControllerBB/BP_BaseAIController.BP_BaseAIController_C|GetAttack%20Target _asbp_base_aicontroller) 5.0 false
        (:then
          (Utilities|FlowControl|Delay 0.25)
          (CallFunction|AttackAnimation)
          (Utilities|FlowControl|Delay 0.5)
          (for _array_element (Collision|GetOverlappingActors (Variables|Default|GetPlayerAttackHitbox) "/Game/Project_West/Game/Character/Blueprints/BP_Character.BP_Character_C" :!class /Script/Engine.PrimitiveComponent)
            (if (Collision|IsOverlappingActor (Variables|Default|GetPlayerAttackHitbox) _array_element :!class /Script/Engine.PrimitiveComponent)
              (Game|Damage|ApplyDamage _array_element (Variables|Default|GetMeleeDamageAmount) 0 0))))))
    (:Is%20Not%20Valid
      (Default|SetStatePassive _asbp_base_aicontroller))))

(fn ConstructionScript
  (|CallParentFunction))

(fn GetIdealRange
  (return 1e+02 3e+02))