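; Base AI controller for enemies that runs the possessed pawn's behavior tree and drives its state through the Blackboard.
; On possess it sets Passive and copies the pawn's attack and defend radii to the Blackboard.
; Perception updates are filtered to player characters; sight or damage triggers Combat and hearing triggers Investigating, only from Passive or Investigating.
; Forgotten targets reset it to Passive, and helper functions set Staggered and UseAbility states.
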(event OnTargetPerceptionForgotten(AIPerception)
  (params (Actor :type Actor%20Object%20Reference))
  (CallFunction|SetStatePassive))

(event OnPerceptionUpdated(AIPerception)
  (params (UpdatedActors :type Array%20of%20Actor%20Object%20References))
  (bind _players (CallFunction|FiltersPlayers UpdatedActors))
  (for _array_element _players
    (Utilities|FlowControl|Sequence
      (:then_0
        (bind _sensed_ (CallFunction|CanSenseActor _array_element "NewEnumerator6"))
        (if _sensed_
          (CallFunction|HandleSensedSight _array_element)))
      (:then_1
        (bind (_sensed__2 _stimulus) (CallFunction|CanSenseActor _array_element "NewEnumerator7"))
        (if _sensed__2
          (CallFunction|HandleSensedSound (.StimulusLocation (Utilities|Struct|BreakAIStimulus _stimulus)))))
      (:then_2
        (bind _sensed__3 (CallFunction|CanSenseActor _array_element "NewEnumerator8"))
        (if _sensed__3
          (CallFunction|HandleSensedDamage _array_element))))))

(event EventPossess
  (params (PossessedPawn :type Pawn%20Object%20Reference))
  (bind _asbp_enemy_base (Utilities|Casting|CastToBP_EnemyBase PossessedPawn))
  (bind _behaviortree (Variables|/Game/Project_West/Game/Enemies/EnemyTypes/BaseClass/BP_EnemyBase.BP_EnemyBase_C|GetBehaviorTree _asbp_enemy_base)
    (:then
      (AI|RunBehaviorTree _behaviortree)
      (CallFunction|SetStatePassive)
      (bind (_attackradius _defendradius) (Class|BPIEnemyAI|GetIdealRange(Message) PossessedPawn))
      (AI|Components|Blackboard|SetValueasFloat (Variables|Default|GetBlackboard) (Variables|Default|GetAttackRadiusKeyname) _attackradius)
      (AI|Components|Blackboard|SetValueasFloat (Variables|Default|GetBlackboard) (Variables|Default|GetDefendRadiusKeyname) _defendradius))
    (:else)))

(fn ConstructionScript)

(fn SetStatePassive
  (AI|Components|Blackboard|SetValueasEnum (Variables|Default|GetBlackboard) (Variables|Default|GetEnum%20KeyName) (Utilities|Enum|LiteralenumE_AIState "NewEnumerator0")))

(fn SetStateCombat
  (params (Atttack%20Target :type Actor%20Object%20Reference) (LastKnownAttackTarget :type Boolean))
  (bind _output_get (Variables|Default|SetAttack%20Target (select LastKnownAttackTarget (Variables|Default|GetAttack%20Target) Atttack%20Target)))
  (Utilities|IsValid _output_get
    (:Is%20Valid
      (AI|Components|Blackboard|SetValueasObject (Variables|Default|GetBlackboard) (Variables|Default|GetTarget%20Keyname) _output_get)
      (AI|Components|Blackboard|SetValueasEnum (Variables|Default|GetBlackboard) (Variables|Default|GetEnum%20KeyName) (Utilities|Enum|LiteralenumE_AIState "NewEnumerator1")))
    (:Is%20Not%20Valid
      (CallFunction|SetStatePassive))))

(fn CanSenseActor
  (params (Actor :type Actor%20Object%20Reference) (SenseType :type E_AISense%20Enum :default "NewEnumerator5"))
  (bind _info (Class|AIPerceptionComponent|GetActorsPerception (Variables|Default|GetAIPerception) Actor))
  (for _array_element (.LastSensedStimuli (Utilities|Struct|BreakActorPerceptionBlueprintInfo _info))
    (bind _returnvalue (Class|AIPerceptionSystem|GetSenseClassforStimulus _array_element))
    (if (== _returnvalue (Utilities|Select :Index SenseType :NewEnumerator5 0 :NewEnumerator6 "/Script/AIModule.AISense_Sight" :NewEnumerator7 "/Script/AIModule.AISense_Hearing" :NewEnumerator8 "/Script/AIModule.AISense_Damage"))
      (return (.bSuccessfullySensed (Utilities|Struct|BreakAIStimulus _array_element)) _array_element))))

(fn HandleSensedSight
  (params (Actor :type Actor%20Object%20Reference))
  (bind _state (CallFunction|GetCurrentState))
  (switch Utilities|FlowControl|Switch|SwitchonE_AIState _state
    (:NewEnumerator0
      _)
    (:NewEnumerator3
      _))
  (CallFunction|SetStateCombat Actor false))

(fn GetCurrentState
  (return (Utilities|Enum|ByteToEnumE_AIState (Class|BlackboardComponent|GetValueasEnum (Variables|Default|GetBlackboard) (Variables|Default|GetEnum%20KeyName)))))

(fn HandleSensedSound
  (params (Location :type Vector))
  (bind _state (CallFunction|GetCurrentState))
  (switch Utilities|FlowControl|Switch|SwitchonE_AIState _state
    (:NewEnumerator0
      _)
    (:NewEnumerator3
      _))
  (CallFunction|SetStateInvestigating Location))

(fn SetStateInvestigating
  (params (Location :type Vector))
  (bind _blackboard (Variables|Default|GetBlackboard))
  (AI|Components|Blackboard|SetValueasEnum _blackboard (Variables|Default|GetEnum%20KeyName) (Utilities|Enum|LiteralenumE_AIState "NewEnumerator3"))
  (AI|Components|Blackboard|SetValueasVector _blackboard (Variables|Default|GetPointOfInterestKeyName) Location))

(fn HandleSensedDamage
  (params (Actor :type Actor%20Object%20Reference))
  (bind _state (CallFunction|GetCurrentState))
  (switch Utilities|FlowControl|Switch|SwitchonE_AIState _state
    (:NewEnumerator0
      _)
    (:NewEnumerator3
      _))
  (CallFunction|SetStateCombat Actor false))

(fn FiltersPlayers
  (params (Actors :type Array%20of%20Actor%20Object%20References))
  (bind _playeractors (Variables|Default|GetPlayerActors))
  (for _array_element Actors
    (bind _asbp_character (Utilities|Casting|CastToBP_Character _array_element))
    (Utilities|Array|Add _playeractors _asbp_character)
    (return _playeractors)))

(fn SetStateasFrozen
  (AI|Components|Blackboard|SetValueasEnum (Variables|Default|GetBlackboard) (Variables|Default|GetEnum%20KeyName) (Utilities|Enum|LiteralenumE_AIState "NewEnumerator2")))

(fn SetStateAbility
  (AI|Components|Blackboard|SetValueasObject (Variables|Default|GetBlackboard) (Variables|Default|GetTarget%20Keyname) 0)
  (AI|Components|Blackboard|SetValueasEnum (Variables|Default|GetBlackboard) (Variables|Default|GetEnum%20KeyName) (Utilities|Enum|LiteralenumE_AIState "NewEnumerator5")))