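; Humanoid shooter enemy that supplies type-specific combat ranges and movement speeds, apparently for a shared enemy framework.
; GetIdealRange returns fixed attack and defend radii, and SetMovementSpeed maps each movement state to a CharacterMovement walk speed, always returning zero.
; Attack and SetVisualState are empty stubs.
; A material swap that would make the mesh emissive in Combat is left unconnected, so it never runs.
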(event EventBeginPlay
  (|CallParentFunction) ; This node is disabled and will not be called.\nDrag off pins to build functionality.
)

(event Collision|EventActorBeginOverlap
  (params (OtherActor :type Actor%20Object%20Reference)))

(event EventTick
  (params (DeltaSeconds :type Float%20%28single-precision%29))
  (|CallParentFunction DeltaSeconds) ; This node is disabled and will not be called.\nDrag off pins to build functionality.
)

(event EventSetVisualState
  (params (NewParam :type E_VisualStates%20Enum :default "NewEnumerator0")))

(event EventAttack)

(fn ConstructionScript
  (|CallParentFunction))

(fn GetIdealRange
  (return 1e+02 3.5e+02))

(fn SetMovementSpeed
  (params (NewParam :type E_MovementSpeed%20Enum :default "NewEnumerator0"))
  (Variables|/Script/Engine.CharacterMovementComponent|SetMaxWalkSpeed (Variables|Character|GetCharacterMovement) (Utilities|Select :Index NewParam :NewEnumerator0 0.0 :NewEnumerator1 3e+02 :NewEnumerator2 4e+02 :NewEnumerator3 5.5e+02 :NewEnumerator4 7e+02))
  (return 0.0))