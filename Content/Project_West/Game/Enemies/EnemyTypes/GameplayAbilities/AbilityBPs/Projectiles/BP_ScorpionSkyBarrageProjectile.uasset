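; Scorpion sky barrage projectile that explodes at the end of a timed move and deals area damage.
; On BeginPlay, the Projectile component moves for two seconds with a fire trail, then spawns explosion effects and sound.
; DamageDeal then hits every actor overlapping DamageCollider except UndamagableActor, with separate maximums for the player and other actors.
; DamageCalculation scales damage down linearly with distance, reaching zero at 1000 units.
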(event Custom|DamageDeal
  (params (Instigator :type Actor%20Object%20Reference))
  (for _array_element (Collision|GetOverlappingActors (Variables|Default|GetDamageCollider) 0 :!class /Script/Engine.PrimitiveComponent)
    (if (== _array_element (Game|GetPlayerCharacter 0))
      (CallFunction|DamageCalculation _array_element _array_element (Variables|Default|GetMaxPlayerDamage) Instigator)
      (elif (not (== _array_element (Variables|Default|GetUndamagableActor)))
        (CallFunction|DamageCalculation _array_element _array_element (Variables|Default|GetMaxEnemy/ObjectDamage) Instigator)))))

(event EventBeginPlay
  (bind _projectile (Variables|Default|GetProjectile))
  (bind _returnvalue (Transformation|GetWorldLocation _projectile))
  (bind _returnvalue_2 (Effects|SpawnEmitterAttached "/Game/StarterContent/Particles/P_Fire.P_Fire" (Variables|Default|GetProjectile) "None"))
  (Components|MoveComponentTo (Variables|Default|GetProjectile) "0, 0, 0" "0.000000,180.000000,180.000000" false false 2.0 false)
  (Components|DestroyComponent _returnvalue_2)
  (Effects|SpawnEmitteratLocation "/Game/StarterContent/Particles/P_Explosion.P_Explosion" _returnvalue "0.000000,180.000000,180.000000")
  (Audio|PlaySoundatLocation "/Game/StarterContent/Audio/Explosion01.Explosion01" _returnvalue "0, 0, 0" 1.0 1.0 0.0 "/Game/Project_West/Game/Level_Hazards/BarrelAttenuation.BarrelAttenuation" 0 0 0)
  (CallFunction|DamageDeal))

(fn ConstructionScript)

(fn DamageCalculation
  (params (DamagedActor :type Actor%20Object%20Reference) (OtherActor :type Actor%20Object%20Reference) (MaxDamage :type Float%20%28double-precision%29) (Instigator :type Actor%20Object%20Reference))
  (Game|Damage|ApplyDamage DamagedActor (Math|Float|Clamp(Float) (* (- 1.0 (/ (Transformation|GetDistanceTo OtherActor) 1e+03)) MaxDamage) 0.0 MaxDamage) 0 0))