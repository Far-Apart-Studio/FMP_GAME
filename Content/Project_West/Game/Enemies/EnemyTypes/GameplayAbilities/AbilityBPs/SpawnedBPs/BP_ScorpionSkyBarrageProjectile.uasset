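; Scorpion sky barrage projectile that runs a timed strike on BeginPlay, hitting in two stages: landing and delayed blast.
; After a delay it moves the projectile component, then plays landing effects and damages Capsule overlaps.
; A second later it clears its visuals, plays the blast and damages DamageCollider overlaps, destroying itself only if it damages something.
; Damage falls off linearly with distance, uses separate player and non-player maximums, and spares UndamagableActor, the damage causer.
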(event Custom|DamageDeal
  (params (Instigator :type Actor%20Object%20Reference))
  ;[1 1 1] DamageDealing
  (for _array_element (Collision|GetOverlappingActors (Variables|Default|GetDamageCollider) 0 :!class /Script/Engine.PrimitiveComponent)
    (if (== _array_element (Game|GetPlayerCharacter 0))
      (CallFunction|DamageCalculation _array_element _array_element (Variables|Default|GetMaxPlayerDamage) Instigator)
      (Utilities|FlowControl|RetriggerableDelay 2.0)
      (Actor|DestroyActor :!label _label)
      (elif (not (== _array_element (Variables|Default|GetUndamagableActor)))
        (CallFunction|DamageCalculation _array_element _array_element (Variables|Default|GetMaxEnemy/ObjectDamage) Instigator)
        (Utilities|FlowControl|RetriggerableDelay 2.0)
        (goto _label)))))

(event Custom|InstantKillDamage
  (params (Instigator :type Actor%20Object%20Reference))
  ;[1 1 1] DamageDealing
  (for _array_element (Collision|GetOverlappingActors (Variables|Default|GetCapsule) 0 :!class /Script/Engine.PrimitiveComponent)
    (if (== _array_element (Game|GetPlayerCharacter 0))
      (CallFunction|DamageCalculation _array_element _array_element (Variables|Default|GetMaxPlayerDamage) Instigator)
      (elif (not (== _array_element (Variables|Default|GetUndamagableActor)))
        (CallFunction|DamageCalculation _array_element _array_element (Variables|Default|GetMaxEnemy/ObjectDamage) Instigator)))))

(event EventBeginPlay
  (bind _projectile (Variables|Default|GetProjectile))
  (bind _returnvalue (Transformation|GetWorldLocation _projectile))
  (Utilities|FlowControl|Delay 1.5)
  (Components|MoveComponentTo (Variables|Default|GetProjectile) "0, 0, 0" "0.000000,180.000000,180.000000" false false 2.0 false)
  (Niagara|SpawnSystematLocation "/Game/Project_West/Assets/Art/VFX/ScorpionBounty/SteamStingerSkyBarrageVFX/VFX/FXS_StingerProjectileLanding.FXS_StingerProjectileLanding" _returnvalue)
  (Audio|PlaySoundatLocation "/Game/StarterContent/Audio/Explosion01.Explosion01" _returnvalue "0, 0, 0" 1.0 1.0 0.0 "/Game/Project_West/Game/Level_Hazards/BarrelAttenuation.BarrelAttenuation" 0 0 0)
  (CallFunction|InstantKillDamage)
  (Utilities|FlowControl|Delay 1.0)
  (Components|DestroyComponent (Variables|Default|GetFXS_StingerProjectile))
  (Niagara|SpawnSystematLocation "/Game/Project_West/Assets/Art/VFX/ScorpionBounty/SteamStingerSkyBarrageVFX/VFX/FXS_StingerProjectileBlast.FXS_StingerProjectileBlast" (Transformation|GetWorldLocation (Variables|Default|GetProjectile)))
  (Audio|PlaySoundatLocation "/Game/StarterContent/Audio/Explosion01.Explosion01" (Transformation|GetWorldLocation (Variables|Default|GetProjectile)) "0, 0, 0" 1.0 1.0 0.0 "/Game/Project_West/Game/Level_Hazards/BarrelAttenuation.BarrelAttenuation" 0 0 0)
  (CallFunction|DamageDeal))

(fn ConstructionScript)

(fn DamageCalculation
  (params (DamagedActor :type Actor%20Object%20Reference) (OtherActor :type Actor%20Object%20Reference) (MaxDamage :type Float%20%28double-precision%29) (Instigator :type Actor%20Object%20Reference))
  (Game|Damage|ApplyDamage DamagedActor (Math|Float|Clamp(Float) (* (- 1.0 (/ (Transformation|GetDistanceTo OtherActor) 1e+03)) MaxDamage) 0.0 MaxDamage) 0 (Variables|Default|GetUndamagableActor)))