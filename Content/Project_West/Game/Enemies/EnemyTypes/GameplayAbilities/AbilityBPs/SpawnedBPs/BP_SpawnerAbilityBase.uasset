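; Base hive spawner for an enemy ability that bursts open and releases mini scorpions, taking its meshes from SpawnerAbilityComponent.
; ActivateHive plays the explode animation and spawns scorpions on the authority at short intervals at SpawnPoint.
; A short delay swaps the hive for its burst mesh and fires explosion effects through Server/Multi events.
; Cooldown, triggered at activation and after spawning, sets the component's OnCooldown flag, then restores the idle hive.
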(event Custom|ParticleSpawnServer
  ;[1 1 1] SpawnsParticles
  (CallFunction|ParticleSpawnMulti))

(event Custom|ParticleSpawnMulti
  (bind _spawnpoint (Variables|Default|GetSpawnPoint))
  (bind _returnvalue (Transformation|GetWorldLocation _spawnpoint))
  ;[1 1 1] SpawnsParticles
  (Effects|SpawnEmitteratLocation "/Game/StarterContent/Particles/P_Explosion.P_Explosion" _returnvalue)
  (Audio|PlaySoundatLocation "/Game/StarterContent/Audio/Explosion01.Explosion01" _returnvalue "0, 0, 0" 1.0 1.0 0.0 "/Game/Project_West/Game/Level_Hazards/BarrelAttenuation.BarrelAttenuation" 0 0 0))

(event Custom|DelayedDisable
  ;[1 1 1] DisablesHive
  (Utilities|FlowControl|Delay 0.53)
  (Rendering|SetVisibility (Variables|Default|GetPW_HiveBurstPH) true false)
  (Rendering|SetVisibility (Variables|Default|GetSK_HivePH) false false)
  (CallFunction|ParticleSpawnServer))

(event Custom|ActivateHive
  ;[1 1 1] ActivatesHive
  (CallFunction|ActivateCooldown)
  (Components|Animation|PlayAnimation (Variables|Default|GetSK_HivePH) "/Game/Project_West/Assets/Animations/Placeholder/Hive/AS_HivePHExplode_Hive_HiveExplode.AS_HivePHExplode_Hive_HiveExplode" false)
  (CallFunction|DelayedDisable)
  (Utilities|ForLoopwithDelay 1 (Variables|Default|GetAmountOfEnemiesToSpawn) 0.25
    (:Output
      (if (Ability|HasAuthority)
        (Game|SpawnActorfromClass "/Game/Project_West/Game/Enemies/EnemyTypes/Scorpion/Blueprints/BP_ScorpionMini.BP_ScorpionMini_C" (Math|Transform|MakeTransform (Transformation|GetWorldLocation (Variables|Default|GetSpawnPoint)) "0, 0, 0" "1.000000,1.000000,1.000000") "Undefined" "MultiplyWithRoot" 0 0)))
    (:Completed
      (CallFunction|ActivateCooldown))))

(event Custom|ResetHive
  ;[1 1 1] ResetsHive
  (Rendering|SetVisibility (Variables|Default|GetPW_HiveBurstPH) false false)
  (Rendering|SetVisibility (Variables|Default|GetSK_HivePH) true false)
  (Components|Animation|PlayAnimation (Variables|Default|GetSK_HivePH) "/Game/Project_West/Assets/Animations/Placeholder/Hive/AS_HivePHExplode_Hive_HiveIdle.AS_HivePHExplode_Hive_HiveIdle" false))

(event Custom|ActivateCooldown
  (bind _spawnerabilitycomponent (Variables|Default|GetSpawnerAbilityComponent))
  ;[1 1 1] ActivatesCooldown
  (Variables|/Game/Project_West/Game/Enemies/EnemyTypes/GameplayAbilities/AbilityComponents/SpawnerAbilityComponent.SpawnerAbilityComponent_C|SetOnCooldown _spawnerabilitycomponent true)
  (Utilities|FlowControl|Delay (Variables|Default|GetCooldownDuration))
  (Variables|/Game/Project_West/Game/Enemies/EnemyTypes/GameplayAbilities/AbilityComponents/SpawnerAbilityComponent.SpawnerAbilityComponent_C|SetOnCooldown _spawnerabilitycomponent false)
  (CallFunction|ResetHive))

(event EventBeginPlay
  (bind _spawnerabilitycomponent (Variables|Default|GetSpawnerAbilityComponent))
  (Components|SkeletalMesh|SetSkeletalMeshAsset (Variables|Default|GetSK_HivePH) (Variables|/Game/Project_West/Game/Enemies/EnemyTypes/GameplayAbilities/AbilityComponents/SpawnerAbilityComponent.SpawnerAbilityComponent_C|GetSkeletalMeshSpawner _spawnerabilitycomponent))
  (Components|StaticMesh|SetStaticMesh (Variables|Default|GetPW_HiveBurstPH) (Variables|/Game/Project_West/Game/Enemies/EnemyTypes/GameplayAbilities/AbilityComponents/SpawnerAbilityComponent.SpawnerAbilityComponent_C|GetStaticMeshSpawner _spawnerabilitycomponent)))

(fn ConstructionScript)