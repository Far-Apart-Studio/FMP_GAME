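; BP_WaveAttack is a spawned enemy ability projectile, a wave that damages and knocks up BP_Character targets.
; Exposed events size the wave's box collider, store a bounty reference and set forward velocity through ProjectileMovement.
; WaveCollider overlaps apply damage and launch the character straight up, overriding existing velocity.
; The actor destroys itself after its lifetime or when DestroyCollider overlaps something.
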(event OnComponentBeginOverlap(WaveCollider)
  (params (OverlappedComponent :type Primitive%20Component%20Object%20Reference) (OtherActor :type Actor%20Object%20Reference) (OtherComp :type Primitive%20Component%20Object%20Reference) (OtherBodyIndex :type Integer) (bFromSweep :type Boolean) (SweepResult :type Hit%20Result%20Structure%20%28by%20ref%29))
  (bind _asbp_character (Utilities|Casting|CastToBP_Character OtherActor))
  (Game|Damage|ApplyDamage _asbp_character (Variables|Default|GetAttackDamage) 0 0)
  (Character|LaunchCharacter _asbp_character "0.000000,0.000000,300.000000" true true))

(event OnComponentBeginOverlap(DestroyCollider)
  (params (OverlappedComponent :type Primitive%20Component%20Object%20Reference) (OtherActor :type Actor%20Object%20Reference) (OtherComp :type Primitive%20Component%20Object%20Reference) (OtherBodyIndex :type Integer) (bFromSweep :type Boolean) (SweepResult :type Hit%20Result%20Structure%20%28by%20ref%29))
  (Actor|DestroyActor))

(event Custom|SetScale
  (params (Width :type Float%20%28double-precision%29) (Length :type Float%20%28double-precision%29) (Height :type Float%20%28double-precision%29) (BountyRef :type Actor%20Object%20Reference))
  (Components|Box|SetBoxExtent (Variables|Default|GetWaveCollider) (Math|Vector|MakeVector Width Length Height) true)
  (Variables|Default|SetBountyRef BountyRef))

(event Custom|MoveForward
  (params (InitialSpeed :type Float%20%28double-precision%29))
  (Variables|/Script/Engine.MovementComponent|SetVelocity (Variables|Default|GetProjectileMovement) (* (Math|Vector|GetForwardVector (Transformation|GetActorRotation)) InitialSpeed)))

(event EventBeginPlay
  (Utilities|FlowControl|Delay 0.1)
  (Utilities|FlowControl|Delay (Variables|Default|GetLifetime))
  (Actor|DestroyActor))

(fn ConstructionScript)