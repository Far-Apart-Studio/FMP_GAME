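; Base enemy character that supplies health feedback, death and helpers for AI states, speeds and random ability selection.
; PWHealth events drive a timed player-facing health bar, damage number actors and a montage stagger that freezes the AI on heavy hits.
; Death plays an animation and unpossesses the controller, while actor destruction waits for a forward material-effect completion.
; Ability cooldown toggles a blackboard key, and Tick manages movement sound.
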(event Custom|StartAbilityCooldown
  (bind _returnvalue (Pawn|GetController))
  (bind _returnvalue_2 (AI|GetBlackboard _returnvalue))
  ;[1 1 1] AbilityCooldown
  (AI|Components|Blackboard|SetValueasBool _returnvalue_2 (Variables|Default|GetCanUseAbility) false)
  (Utilities|FlowControl|Delay (Variables|Default|GetAbilityDelay))
  (AI|Components|Blackboard|SetValueasBool _returnvalue_2 (Variables|Default|GetCanUseAbility) true))

(event Custom|_onHighlightComplete_Event
  (params (Direction :type EEffectDirection%20Enum :default "ED_Forward"))
  ;[1 1 1] Assigning events/Death Handling
  (if (Utilities|Enum|Equal(Enum) Direction "ED_Forward")
    (Actor|DestroyActor)))

(event Custom|DeathEvent
  ;[1 1 1] Assigning events/Death Handling
  (CallFunction|EnemyDeath))

(event Custom|DeathEventServer
  ;[1 1 1] Assigning events/Death Handling
  (CallFunction|DeathEvent))

(event Custom|HealthChanged
  ;[1 1 1] Assigning events/Death Handling
  (CallFunction|DamageDealtBind)
  (CallFunction|ChangeHealtbarVariable)
  (CallFunction|HealthbarTrigger)
  (Default|HitAnimation (Variables|Default|GetHealthbarWidget))
  (if (Variables|Default|GetCanBeStaggered)
    (Components|Movement|StopMovementImmediately (Variables|Character|GetCharacterMovement))
    (if (> (Variables|Default|GetDamageDealt) 3e+01)
      (Default|SetStateasFrozen (Variables|Default|GetBP%20Base%20AIController))
      (Animation|Montage|PlayMontage (Variables|Character|GetMesh) (Variables|Default|GetHitReaction) 2.0
        (:OnCompleted
          _)
        (:OnInterrupted
          _))
      (Default|SetStateCombat (Variables|Default|GetBP%20Base%20AIController) 0 true))))

(event Custom|OnDeathEvent
  (params (OwnerActor :type Actor%20Object%20Reference) (DamageCauser :type Actor%20Object%20Reference) (DamageCauserController :type Controller%20Object%20Reference))
  ;[1 1 1] Assigning events/Death Handling
  (CallFunction|DeathEventServer))

(event Custom|HealthbarTrigger
  ;[1 1 1] HealthBar
  (Variables|Default|SetHealthbarEnabled true)
  (CallFunction|ShowHealthBar)
  (Utilities|FlowControl|RetriggerableDelay 5.0)
  (CallFunction|RemoveHealthBar)
  (Utilities|FlowControl|RetriggerableDelay 6.5)
  (Variables|Default|SetHealthbarEnabled false))

(event Custom|StartingHP
  ;[1 1 1] DamageNumbers
  (Variables|Default|SetCurrentHealth (Variables|/Script/PROJECT_WEST.PW_HealthComponent|Get_currentHealth (Variables|Default|GetPW_Health))))

(event Custom|DamageDealtBind
  ;[1 1 1] DamageNumbers
  (CallFunction|DamageTaken))

(event Custom|EnemyMovingSounds
  ;[1 1 1] EnemyMovingSound
  (if (> (Math|Vector|VectorLength (Variables|/Script/Engine.MovementComponent|GetVelocity (Variables|Character|GetCharacterMovement))) 1e+01)
    (Utilities|FlowControl|DoOnce false :!label _label
      (:Completed
        (bind _returnvalue (Audio|SpawnSoundAttached (Variables|Default|GetMovingSound) (Variables|Character|GetMesh) "None" "0, 0, 0" "0, 0, 0" "KeepRelativeOffset" false 1.0 1.0 0.0 "/Game/Project_West/Game/Level_Hazards/BarrelAttenuation.BarrelAttenuation" 0))))
    (else
      (Utilities|IsValid _returnvalue
        (:Is%20Valid
          (Audio|Components|Audio|Stop _returnvalue)
          (Components|DestroyComponent _returnvalue)
          (goto _label Reset))))))

(event EventTick
  (params (DeltaSeconds :type Float%20%28single-precision%29))
  ;[1 1 1] TickEvent
  (CallFunction|HealthbarLookatPlayer)
  (CallFunction|EnemyMovingSounds))

(event EventBeginPlay
  ;[1 1 1] BeginPlay
  (AI|Components|Blackboard|SetValueasBool (AI|GetBlackboard (Pawn|GetController)) (Variables|Default|GetCanUseAbility) true)
  (CallFunction|BeginGenerateValues)
  ;[1 1 1] Assigning events/Death Handling
  (EventDispatchers|AssignOnDeath (Variables|Default|GetPW_Health) (delegate Custom|OnDeathEvent))
  (EventDispatchers|AssignOnHealthChanged (Variables|Default|GetPW_Health) (delegate Custom|HealthChanged))
  (EventDispatchers|BindEventtoOnHighlightComplete (Variables|Default|GetPW_MaterialEffect) (delegate Custom|_onHighlightComplete_Event)))

(event EventSetVisualState
  (params (NewParam :type E_VisualStates%20Enum :default "NewEnumerator0"))
  (Rendering|Material|SetMaterial (Variables|Character|GetMesh) 0 (Utilities|Select :Index NewParam :NewEnumerator0 "/Game/ExternalAssets/Scorpio/Materials/Gold/M_Light.M_Light" :NewEnumerator1 "/Game/SteamPunkCollection/SteamPunkAndroid/Materials/Character/M_Light.M_Light" :NewEnumerator2 "/Game/Project_West/Temp/TB/Emissive.Emissive")))

(fn ConstructionScript)

(fn ShowHealthBar
  (Default|EnableHealthbar (Variables|Default|GetHealthbarWidget)))

(fn RemoveHealthBar
  (Default|FadeOutHealthBar (Variables|Default|GetHealthbarWidget)))

(fn GetEnemyMaxHP
  (Variables|/Game/Project_West/Game/Enemies/W_EnemyHealthbar.W_EnemyHealthbar_C|SetMaxHealth (Variables|Default|GetHealthbarWidget) (Variables|/Script/PROJECT_WEST.PW_HealthComponent|Get_maxHealth (Variables|Default|GetPW_Health))))

(fn ChangeHealtbarVariable
  (bind _healthbarwidget (Variables|Default|GetHealthbarWidget))
  (bind _pw_health (Variables|Default|GetPW_Health))
  (bind _output_get (Variables|/Game/Project_West/Game/Enemies/W_EnemyHealthbar.W_EnemyHealthbar_C|SetHealth _healthbarwidget (Variables|/Script/PROJECT_WEST.PW_HealthComponent|Get_currentHealth _pw_health)))
  (Default|SetHealth _healthbarwidget (Math|Float|Clamp(Float) (/ _output_get (Variables|/Script/PROJECT_WEST.PW_HealthComponent|Get_maxHealth _pw_health)))))

(fn WidgetCast
  (bind _asw_enemy_healthbar (Utilities|Casting|CastToW_EnemyHealthbar (UserInterface|GetWidget (Variables|Default|GetHealthbar))))
  (Variables|Default|SetHealthbarWidget _asw_enemy_healthbar))

(fn GetPlayerRef
  (bind _outactors (Actor|GetAllActorsOfClass "/Script/PROJECT_WEST.PW_Character"))
  (Variables|Default|SetPlayerVar (Utilities|Array|Get(acopy) _outactors)))

(fn HealthbarLookatPlayer
  (if (Variables|Default|GetHealthbarEnabled)
    (Transformation|SetWorldRotation (Variables|Default|GetHealthbar) (Math|Rotator|FindLookatRotation (Transformation|GetWorldLocation (Variables|Default|GetHealthbar)) (Transformation|GetActorLocation (Variables|Default|GetPlayerVar))) false false)))

(fn DamageDealtFunction
  (params (self2 :type PW%20Health%20Component%20Object%20Reference))
  (bind __currenthealth (Variables|/Script/PROJECT_WEST.PW_HealthComponent|Get_currentHealth self2))
  (Variables|Default|SetDamageDealt (- (Variables|Default|GetCurrentHealth) __currenthealth))
  (Variables|Default|SetCurrentHealth __currenthealth)
  (return __currenthealth))

(fn DamageTaken
  (CallFunction|DamageDealtFunction (Variables|Default|GetPW_Health))
  (bind _returnvalue (Game|SpawnActorfromClass "/Game/Project_West/Game/Enemies/DamageNumberWidget.DamageNumberWidget_C" (Transformation|GetWorldTransform (Variables|Default|GetHealthbar)) "Undefined" "MultiplyWithRoot" 0 0))
  (Variables|/Game/Project_West/Game/Enemies/DamageNumberWidget.DamageNumberWidget_C|SetDamageAmount _returnvalue (Math|Float|Truncate (Variables|Default|GetDamageDealt))))

(fn EnemyDeath
  (Components|Animation|PlayAnimation (Variables|Character|GetMesh) "/Game/Project_West/Assets/Animations/Enemy_Animations/Steamstinger_Animations/AnimationSequences/AS_Steamstinger_Death.AS_Steamstinger_Death" false)
  (Pawn|Components|CharacterMovement|DisableMovement (Variables|Character|GetCharacterMovement))
  (Variables|Default|SetDead true)
  (Collision|SetCollisionEnabled (Variables|Collision|GetCapsuleComponent) "QueryOnly")
  (Rendering|SetVisibility (Variables|Default|GetHealthbar) false false)
  (Pawn|UnPossess (Pawn|GetController)))

(fn BeginGenerateValues
  (CallFunction|WidgetCast)
  (CallFunction|GetEnemyMaxHP)
  (CallFunction|ChangeHealtbarVariable)
  (CallFunction|GetPlayerRef)
  (CallFunction|StartingHP)
  (Class|PWMaterialEffectComponent|ActivateEffect (Variables|Default|GetPW_MaterialEffect) "ED_Backward")
  (bind _asbp_base_aicontroller (Utilities|Casting|CastToBP_BaseAIController (AI|GetAIController self)))
  (Variables|Default|SetBP%20Base%20AIController _asbp_base_aicontroller))

(fn GenerateAbilities
  (for _index (range 1 (Variables|Ability|GetMaxAmountOfAbilities))
    (bind _output_get (LocalVariables|SetRemovedItem (.OutItem (Utilities|Array|Random (Variables|Ability|GetAvailableAbilities)))))
    (Utilities|Array|Add (Variables|Ability|GetChosenAbilities) _output_get)
    (Utilities|Array|RemoveItem (Variables|Ability|GetAvailableAbilities) _output_get)))

(fn GetAbility
  (bind _output_get (Variables|Ability|SetSelectedAbility (.OutItem (Utilities|Array|Random (Variables|Ability|GetChosenAbilities)))))
  (return _output_get))

(fn GetIdealRange
  (return 1.5e+02 4.5e+02))

(fn SetMovementSpeed
  (params (NewParam :type E_MovementSpeed%20Enum :default "NewEnumerator0"))
  (bind _output_get (Variables|/Script/Engine.CharacterMovementComponent|SetMaxWalkSpeed (Variables|Character|GetCharacterMovement) (Utilities|Select :Index NewParam :NewEnumerator0 0.0 :NewEnumerator1 375.0 :NewEnumerator2 575.0 :NewEnumerator3 675.0 :NewEnumerator4 9e+02)))
  (return _output_get))