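; Base scorpion grunt enemy that roams around its spawn point and chases players when in range or damaged.
; Tick picks the nearest living player on the navmesh as the target for AI movement, delayed-hitbox melee and random, line-of-sight-checked projectiles.
; Externally triggered attack events share cooldown and death checks.
; PWHealth events drive chasing, a temporary player-facing healthbar, floating damage numbers and death, while PWMaterialEffect completion handles destruction.
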(event Custom|Attack
  ;[1 1 1] Attack Event
  (CallFunction|MultiAttack))

(event Custom|MultiAttack
  ;[1 1 1] Attack Event
  (if (not (Variables|Default|GetDead))
    (if (not (Variables|Default|GetAttackCooldown))
      (Variables|Default|SetAttacking true)
      (Variables|Default|SetAttackCooldown true)
      (Audio|PlaySoundatLocation "/Game/Project_West/Assets/Audio/SFX/Enemies/Grunt/MeleeAttack.MeleeAttack" (Transformation|GetActorLocation) "0, 0, 0" 1.0 1.0 0.0 "/Game/Project_West/Game/Level_Hazards/BarrelAttenuation.BarrelAttenuation" 0 0 0)
      (Animation|PlayAnimMontage "/Game/Project_West/Game/Enemies/Bounties/Steamstinger/Animations/PrototypeAttack.PrototypeAttack" 1.0 "None")
      (Utilities|FlowControl|Delay 0.3)
      (if (Collision|IsOverlappingActor (Variables|Default|GetPlayerAttackHitbox) (Variables|Default|GetClosestPlayerAI) :!class /Script/Engine.PrimitiveComponent)
        (Game|Damage|ApplyDamage (Variables|Default|GetClosestPlayerAI) (Variables|Default|GetMeleeDamageAmount) 0 0)
        (Audio|PlaySoundatLocation "/Game/Project_West/Assets/Audio/SFX/Character/Hit/MeleeHit.MeleeHit" (Transformation|GetActorLocation (Variables|Default|GetClosestPlayerAI)) "0, 0, 0" 0.75 0.75 0.35 "/Game/Project_West/Game/Level_Hazards/BarrelAttenuation.BarrelAttenuation" 0 0 0)
        (Utilities|FlowControl|Delay 0.8)
        (Variables|Default|SetAttackCooldown false)
        (else
          (Utilities|FlowControl|Delay 0.8)
          (Variables|Default|SetAttackCooldown false))))))

(event Custom|MultiHit
  ;[1 1 1] Hit By Player
  (Animation|Montage|PlayMontage (Variables|Character|GetMesh) "/Game/Project_West/Game/Enemies/Bounties/Steamstinger/Animations/AM_ScorpionHit.AM_ScorpionHit"))

(event Custom|_onHighlightComplete_Event
  (params (Direction :type EEffectDirection%20Enum :default "ED_Forward"))
  ;[1 1 1] Assigning events/Death Handling
  (if (Utilities|Enum|Equal(Enum) Direction "ED_Forward")
    (Actor|DestroyActor)))

(event Custom|DeathEvent
  ;[1 1 1] Assigning events/Death Handling
  (Components|Animation|PlayAnimation (Variables|Character|GetMesh) "/Game/ExternalAssets/Scorpio/Animations/Anim_Scorpio_Death.Anim_Scorpio_Death" false)
  (Pawn|Components|CharacterMovement|DisableMovement (Variables|Character|GetCharacterMovement))
  (Variables|Default|SetDead true)
  (Collision|SetCollisionEnabled (Variables|Collision|GetCapsuleComponent) "QueryOnly")
  (Rendering|SetVisibility (Variables|Default|GetHealthbar) false false))

(event Custom|DeathEventServer
  ;[1 1 1] Assigning events/Death Handling
  (CallFunction|DeathEvent))

(event Custom|HealthChanged
  ;[1 1 1] Assigning events/Death Handling
  (CallFunction|ChaseonDamage)
  (CallFunction|DamageDealtBind)
  (CallFunction|ChangeHealtbarVariable)
  (CallFunction|HealthbarTrigger)
  (Default|HitAnimation (Variables|Default|GetHealthbarWidget)))

(event Custom|GetSpawnLocation
  ;[1 1 1] GetSpawnPoint
  (Utilities|FlowControl|Delay 0.1)
  (Variables|Default|SetSpawnLocation (Transformation|GetActorLocation))
  (CallFunction|RandomRoam))

(event Custom|ChaseOnDamage
  (bind _closestplayerai (Variables|Default|GetClosestPlayerAI))
  ;[1 1 1] ChasePlayersWhenDamaged
  (Effects|SpawnEmitteratLocation "/Game/StarterContent/Particles/P_Explosion.P_Explosion" (Transformation|GetWorldLocation (Variables|Default|GetScene)))
  (if (not (Variables|Default|GetChasing))
    (Variables|Default|SetChasing true)
    (CallFunction|MovetoPlayers)
    (Utilities|FlowControl|RetriggerableDelay 1e+01 :!label _label)
    (Utilities|IsValid _closestplayerai
      (:Is%20Valid
        (if (>= (Transformation|GetDistanceTo _closestplayerai self) 2e+03)
          (Variables|Default|SetChasing false)
          (else
            (goto _label)))))))

(event Custom|OnDeathEvent
  (params (OwnerActor :type Actor%20Object%20Reference) (DamageCauser :type Actor%20Object%20Reference) (DamageCauserController :type Controller%20Object%20Reference))
  ;[1 1 1] Assigning events/Death Handling
  (CallFunction|DeathEventServer))

(event Custom|RandomRoam
  ;[1 1 1] Random Roaming
  (if (not (Variables|Default|GetChasing))
    (if (not (Variables|Default|GetInRange))
      (bind _randomlocation (Class|NavigationSystemV1|GetRandomLocationinNavigableRadius (Variables|Default|GetSpawnLocation) (Variables|Default|GetRoamRadius) 0 0))
      (AI|AIMoveTo self _randomlocation 0 5e+01 false
        (:OnSuccess
          (Utilities|FlowControl|Delay (Math|Random|RandomFloatinRange 8.0 12.0))
          (if (not (Variables|Default|GetChasing))
            (CallFunction|RandomRoam)))
        (:OnFail
          (CallFunction|RandomRoam))))))

(event Custom|HealthbarTrigger
  ;[1 1 1] HealthBar
  (Variables|Default|SetHealthbarEnabled true)
  (CallFunction|ShowHealthBar)
  (Utilities|FlowControl|RetriggerableDelay 5.0)
  (CallFunction|RemoveHealthBar)
  (Utilities|FlowControl|RetriggerableDelay 6.5)
  (Variables|Default|SetHealthbarEnabled false))

(event Custom|StartingHP
  ;[1 1 1] DamageNumbers
  (Variables|Default|SetCurrentHealth (Variables|/Script/PROJECT_WEST.PW_HealthComponent|Get_currentHealth (Variables|Default|GetPW_Health))))

(event Custom|DamageDealtBind
  ;[1 1 1] DamageNumbers
  (CallFunction|DamageTaken))

(event Custom|EnemyMovingSounds
  ;[1 1 1] EnemyMovingSound
  (if (> (Math|Vector|VectorLength (Variables|/Script/Engine.MovementComponent|GetVelocity (Variables|Character|GetCharacterMovement))) 1e+01)
    (Utilities|FlowControl|DoOnce false :!label _label
      (:Completed
        (bind _returnvalue (Audio|SpawnSoundAttached "/Game/Project_West/Assets/Audio/SFX/Enemies/Grunt/CritterMovingSound.CritterMovingSound" (Variables|Character|GetMesh) "None" "0, 0, 0" "0, 0, 0" "KeepRelativeOffset" false 1.0 1.0 0.0 "/Game/Project_West/Game/Level_Hazards/BarrelAttenuation.BarrelAttenuation" 0))))
    (else
      (Utilities|IsValid _returnvalue
        (:Is%20Valid
          (Audio|Components|Audio|Stop _returnvalue)
          (Components|DestroyComponent _returnvalue)
          (goto _label Reset))))))

(event Custom|MoveToPlayers
  ;[1 1 1] Move to player/Get players location
  (|MoveToPlayer))

(event Custom|HitByPlayer
  ;[1 1 1] Hit By Player
  (CallFunction|MultiHit))

(event Custom|ShootAttack
  ;[1 1 1] Shooting
  (CallFunction|DistanceCheck)
  (if (Variables|Default|GetRangedAttackDistance)
    (CallFunction|MultiShoot)))

(event Custom|MultiShoot
  ;[1 1 1] Shooting
  (if (Variables|Default|GetCanShoot)
    (if (not (Variables|Default|GetDead))
      (CallFunction|Shooting)
      (if (Variables|Default|GetShootingCD)
        (Utilities|FlowControl|Delay 5.0)
        (Variables|Default|SetShootingCD false)))))

(event EventTick
  (params (DeltaSeconds :type Float%20%28single-precision%29))
  ;[1 1 1] CheckingClosestPlayers
  (CallFunction|GettingClosestPlayer)
  (CallFunction|HealthbarLookatPlayer)
  (CallFunction|EnemyMovingSounds))

(event EventBeginPlay
  ;[1 1 1] BeginPlay
  (CallFunction|WidgetCast)
  (CallFunction|GetSpawnLocation)
  (CallFunction|GetEnemyMaxHP)
  (CallFunction|ChangeHealtbarVariable)
  (CallFunction|GetPlayerRef)
  (CallFunction|StartingHP)
  (Class|PWMaterialEffectComponent|ActivateEffect (Variables|Default|GetPW_MaterialEffect) "ED_Backward")
  ;[1 1 1] Assigning events/Death Handling
  (EventDispatchers|AssignOnDeath (Variables|Default|GetPW_Health) (delegate Custom|OnDeathEvent))
  (EventDispatchers|AssignOnHealthChanged (Variables|Default|GetPW_Health) (delegate Custom|HealthChanged))
  (EventDispatchers|BindEventtoOnHighlightComplete (Variables|Default|GetPW_MaterialEffect) (delegate Custom|_onHighlightComplete_Event)))

(fn ConstructionScript)

(fn Shooting
  (bind _scene (Variables|Default|GetScene))
  (bind _returnvalue (Transformation|GetWorldLocation _scene))
  (if (Variables|Default|GetCanShoot)
    (Utilities|IsValid (Variables|Default|GetClosestPlayerAI)
      (:Is%20Valid
        (bind _outhit (Collision|LineTraceByChannel (Transformation|GetActorLocation) (Transformation|GetActorLocation (Variables|Default|GetClosestPlayerAI)) "TraceTypeQuery1" false 0 "None"))
        (if (== (.HitActor (Collision|BreakHitResult _outhit)) (Variables|Default|GetPlayerVar))
          (if (not (Variables|Default|GetDead))
            (if (Variables|Default|GetChasing)
              (if (not (Variables|Default|GetShootingCD)) :!label _label
                (if (> (Math|Random|RandomFloatinRange 1.0 1e+02) 97.0)
                  (Variables|Default|SetShootingCD true)
                  (Game|SpawnActorfromClass "/Game/Project_West/Temp/TB/BP_PrototypeAIProjectile.BP_PrototypeAIProjectile_C" (Math|Transform|MakeTransform _returnvalue (Math|Rotator|FindLookatRotation _returnvalue (Transformation|GetActorLocation (Variables|Default|GetClosestPlayerAI))) "1.000000,1.000000,1.000000") "Undefined" "MultiplyWithRoot" 0 0)
                  (Audio|PlaySoundatLocation "/Game/StarterContent/Audio/Explosion02.Explosion02" (Transformation|GetActorLocation) "0, 0, 0" 0.75 1.0 0.0 "/Game/Project_West/Game/Level_Hazards/BarrelAttenuation.BarrelAttenuation" 0 0 0)))
              (elif (Variables|Default|GetInRange)
                (goto _label)))))))))

(fn DistanceCheck
  (bind _aspw_character (Utilities|Casting|CastToPW_Character (Game|GetPlayerCharacter 0)))
  (if (> (Transformation|GetDistanceTo _aspw_character) 6e+02)
    (Variables|Default|SetRangedAttackDistance true)
    (else
      (Variables|Default|SetRangedAttackDistance false))))

(fn GetActorsonNavmesh
  (bind _actorarray (LocalVariables|GetActorArray))
  (bind _outactors (Actor|GetAllActorsOfClass "/Script/PROJECT_WEST.PW_Character"))
  (for _array_element _outactors
    (if (AI|IsValidAILocation (Transformation|GetActorLocation _array_element))
      (bind _aspw_character (Utilities|Casting|CastToPW_Character _array_element))
      (if (Class|PWCharacter|IsAlive _aspw_character)
        (Utilities|Array|Add _actorarray _array_element))))
  (return _actorarray))

(fn GettingClosestPlayer
  (if (not (Variables|Default|GetDead))
    (bind _onnavmesh (CallFunction|GetActorsonNavmesh))
    (for (_array_element _array_index) _onnavmesh
      (if (== _array_index 0)
        (Variables|Default|SetCurrentClosestDistance (Transformation|GetDistanceTo self _array_element))
        (Variables|Default|SetClosestPlayerAI _array_element)
        (elif (< (Transformation|GetDistanceTo self _array_element) (Variables|Default|GetCurrentClosestDistance))
          (Variables|Default|SetCurrentClosestDistance (Transformation|GetDistanceTo self _array_element))
          (Variables|Default|SetClosestPlayerAI _array_element))))))

(fn ShowHealthBar
  (Default|EnableHealthbar (Variables|Default|GetHealthbarWidget)))

(fn RemoveHealthBar
  (Default|FadeOutHealthBar (Variables|Default|GetHealthbarWidget)))

(fn GetEnemyMaxHP
  (Variables|/Game/Project_West/Game/Enemies/W_EnemyHealthbar.W_EnemyHealthbar_C|SetMaxHealth (Variables|Default|GetHealthbarWidget) (Variables|/Script/PROJECT_WEST.PW_HealthComponent|Get_maxHealth (Variables|Default|GetPW_Health))))

(fn ChangeHealtbarVariable
  (bind _healthbarwidget (Variables|Default|GetHealthbarWidget))
  (bind _pw_health (Variables|Default|GetPW_Health))
  (bind _output_get (Variables|/Game/Project_West/Game/Enemies/W_EnemyHealthbar.W_EnemyHealthbar_C|SetHealth _healthbarwidget (Variables|/Script/PROJECT_WEST.PW_HealthComponent|Get_currentHealth _pw_health)))
  (Default|SetHealth _healthbarwidget (Math|Float|Clamp(Float) (/ _output_get (Variables|/Script/PROJECT_WEST.PW_HealthComponent|Get_maxHealth _pw_health)))))

(fn WidgetCast
  (bind _asw_enemy_healthbar (Utilities|Casting|CastToW_EnemyHealthbar (UserInterface|GetWidget (Variables|Default|GetHealthbar))))
  (Variables|Default|SetHealthbarWidget _asw_enemy_healthbar))

(fn GetPlayerRef
  (bind _outactors (Actor|GetAllActorsOfClass "/Script/PROJECT_WEST.PW_Character"))
  (Variables|Default|SetPlayerVar (Utilities|Array|Get(acopy) _outactors)))

(fn HealthbarLookatPlayer
  (if (Variables|Default|GetHealthbarEnabled)
    (Transformation|SetWorldRotation (Variables|Default|GetHealthbar) (Math|Rotator|FindLookatRotation (Transformation|GetWorldLocation (Variables|Default|GetHealthbar)) (Transformation|GetActorLocation (Variables|Default|GetPlayerVar))) false false)))

(fn DamageDealtFunction
  (params (self2 :type PW%20Health%20Component%20Object%20Reference))
  (bind __currenthealth (Variables|/Script/PROJECT_WEST.PW_HealthComponent|Get_currentHealth self2))
  (Variables|Default|SetDamageDealt (- (Variables|Default|GetCurrentHealth) __currenthealth))
  (Variables|Default|SetCurrentHealth __currenthealth)
  (return __currenthealth))

(fn DamageTaken
  (CallFunction|DamageDealtFunction (Variables|Default|GetPW_Health))
  (bind _returnvalue (Game|SpawnActorfromClass "/Game/Project_West/Game/Enemies/DamageNumberWidget.DamageNumberWidget_C" (Transformation|GetWorldTransform (Variables|Default|GetHealthbar)) "Undefined" "MultiplyWithRoot" 0 0))
  (Variables|/Game/Project_West/Game/Enemies/DamageNumberWidget.DamageNumberWidget_C|SetDamageAmount _returnvalue (Math|Float|Truncate (Variables|Default|GetDamageDealt))))