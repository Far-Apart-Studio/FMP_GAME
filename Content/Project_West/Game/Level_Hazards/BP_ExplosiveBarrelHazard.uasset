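; Explosive barrel level hazard that catches fire when damaged to low health and explodes on death.
; At low health a looping timer drains its health while fire effects play.
; Death passes through server and multicast events to explode, applying distance-scaled damage to overlapping actors, with a separate maximum for the first player.
; The barrel destroys itself only if valid fire effects exist to clean up.
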(event Custom|Multicast
  (CallFunction|BarrelDeath (stale Custom|OnDamageReceivedGlobal_Event _returnvalue_3) (stale Custom|OnDamageReceivedGlobal_Event _returnvalue_4))
  (Utilities|Time|ClearandInvalidateTimerbyHandle (stale Custom|OnDamageReceivedGlobal_Event _returnvalue_2)))

(event Custom|RunOnServer
  (CallFunction|Multicast))

(event Custom|OnDeathEvent
  (params (OwnerActor :type Actor%20Object%20Reference) (DamageCauser :type Actor%20Object%20Reference) (DamageCauserController :type Controller%20Object%20Reference))
  (CallFunction|RunonServer))

(event Custom|OnDamageReceivedGlobal_Event
  (params (OwnerActor :type Actor%20Object%20Reference) (DamageCauser :type Actor%20Object%20Reference) (DamageCauserController :type Controller%20Object%20Reference) (DamageAmount :type Float%20%28single-precision%29))
  (bind _scene (Variables|Default|GetScene))
  (bind _returnvalue (Transformation|GetWorldLocation _scene))
  (CallFunction|HealthCheck)
  (if (Variables|Default|GetStartDrain)
    (bind _returnvalue_2 (Utilities|Time|SetTimerbyFunctionName 0 "HealthDrain" 1.0 true))
    (Utilities|FlowControl|DoOnce false
      (:Completed
        (bind _returnvalue_3 (Effects|SpawnEmitteratLocation "/Game/StarterContent/Particles/P_Fire.P_Fire" _returnvalue))
        (bind _returnvalue_4 (Audio|SpawnSoundatLocation "/Game/StarterContent/Audio/Fire01_Cue.Fire01_Cue" _returnvalue "0, 0, 0" 1.0 1.0 0.0 "/Game/Project_West/Game/Level_Hazards/BarrelAttenuation.BarrelAttenuation" 0))))))

(event EventBeginPlay
  (bind _pw_health (Variables|Default|GetPW_Health))
  (EventDispatchers|AssignOnDeathGlobal _pw_health (delegate Custom|OnDeathEvent))
  (EventDispatchers|AssignOnDamageReceivedGlobal _pw_health (delegate Custom|OnDamageReceivedGlobal_Event)))

(fn ConstructionScript)

(fn DamageCalculation
  (params (DamagedActor :type Actor%20Object%20Reference) (OtherActor :type Actor%20Object%20Reference) (MaxDamage :type Float%20%28double-precision%29))
  (Game|Damage|ApplyDamage DamagedActor (Math|Float|Clamp(Float) (* (- 1.0 (/ (Transformation|GetDistanceTo OtherActor) 1e+03)) MaxDamage) 0.0 MaxDamage) 0 self))

(fn BarrelDamage
  (for _array_element (Collision|GetOverlappingActors (Variables|Default|GetDamageCollider) 0 :!class /Script/Engine.PrimitiveComponent)
    (if (== _array_element (Game|GetPlayerCharacter 0))
      (CallFunction|DamageCalculation _array_element _array_element (Variables|Default|GetMaxPlayerDamage))
      (else
        (CallFunction|DamageCalculation _array_element _array_element (Variables|Default|GetMaxEnemy/Object%20Damage))))))

(fn HealthCheck
  (if (<= (Variables|/Script/PROJECT_WEST.PW_HealthComponent|Get_currentHealth (Variables|Default|GetPW_Health)) 35.0)
    (Variables|Default|SetStartDrain true)))

(fn HealthDrain
  (bind _self self)
  (Game|Damage|ApplyDamage _self (Variables|Default|GetDrainAmount/Second) 0 _self))

(fn BarrelDeath
  (params (self2 :type Actor%20Component%20Object%20Reference) (self3 :type Audio%20Component%20Object%20Reference))
  (Effects|SpawnEmitteratLocation "/Game/StarterContent/Particles/P_Explosion.P_Explosion" (Transformation|GetWorldLocation (Variables|Default|GetBarrel)) "0, 0, 0" "2.000000,2.000000,2.000000")
  (Audio|PlaySoundatLocation "/Game/StarterContent/Audio/Explosion_Cue.Explosion_Cue" (Transformation|GetWorldLocation (Variables|Default|GetBarrel)) "0, 0, 0" 1.0 1.0 0.0 "/Game/Project_West/Game/Level_Hazards/BarrelAttenuation.BarrelAttenuation" 0 0 0)
  (CallFunction|BarrelDamage)
  (Utilities|IsValid self2
    (:Is%20Valid
      (Utilities|IsValid self3
        (:Is%20Valid
          (Components|DestroyComponent self2)
          (Audio|Components|Audio|Stop self3)
          (Actor|DestroyActor))))))