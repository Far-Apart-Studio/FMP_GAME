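; BP_CompassLocator puts a compass HUD on the player's screen and marks active side objectives on it.
; SetUp resolves and caches the local PW_Character through the game state, then creates the compass widget for its controller.
; It then adds an icon per objective from BP_SideObjectiveManager, chosen by task type and targeting its POI area.
; RemoveTaskFromCompass clears an objective's marker using that area.
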(fn SetUp
  (bind _character (CallFunction|GetCharacter))
  (bind _asbp_player_controller (Utilities|Casting|CastToBP_PlayerController (Pawn|GetController _character)))
  (bind _output_get (Variables|Default|SetPlayer%20Controller%20BP _asbp_player_controller))
  (bind _returnvalue (UserInterface|CreateWidget "/Game/Project_West/Game/Compass/BP_CompassHUD.BP_CompassHUD_C" _output_get))
  (bind _output_get_2 (Variables|Default|SetCompassHUD _returnvalue))
  (UserInterface|Viewport|AddtoViewport _output_get_2 0)
  (CallFunction|AddTaskstoCompass))

(fn AddTaskstoCompass
  (bind _returnvalue (Actor|GetActorOfClass "/Game/Project_West/Game/SideObjectives/BP_SideObjectiveManager.BP_SideObjectiveManager_C"))
  (Utilities|IsValid _returnvalue
    (:Is%20Valid
      (for _array_element (Variables|/Script/PROJECT_WEST.PW_SideObjectiveManager|Get_activeObjectives _returnvalue)
        (bind _returnvalue_2 (UserInterface|CreateWidget "/Game/Project_West/Game/Compass/BP_Compass_Icon.BP_Compass_Icon_C"))
        (Default|SetUp _returnvalue_2 (Utilities|Select :Index (._taskType (Utilities|Struct|BreakSideObjectiveEntry (Variables|/Script/PROJECT_WEST.PW_SideObjective|Get_objectiveData _array_element))) :EElimination "/Game/Project_West/Game/Compass/Compass_Icon2.Compass_Icon2" :EDemolition "/Game/Project_West/Game/Compass/Compass_Icon1.Compass_Icon1" :ECollection "/Game/Project_West/Game/Compass/Compass_Icon3.Compass_Icon3") (Variables|/Script/PROJECT_WEST.PW_SideObjective|Get_poiArea _array_element) (Variables|Default|GetPW_Character))
        (Default|AddCompassLocation (Variables|Default|GetCompassHUD) _returnvalue_2)))))

(fn GetCharacter
  (Utilities|IsValid (Variables|Default|GetPW_Character)
    (:Is%20Valid
      (return (Variables|Default|GetPW_Character)))
    (:Is%20Not%20Valid
      (bind _aspw_game_state (Utilities|Casting|CastToPW_GameState (Game|GetGameState)))
      (bind _returnvalue (Class|PWGameState|GetLocalPlayerController _aspw_game_state))
      (bind _aspw_character (Utilities|Casting|CastToPW_Character (Pawn|GetControlledPawn _returnvalue)))
      (bind _output_get (Variables|Default|SetPW_Character _aspw_character))
      (return _output_get))))

(fn RemoveTaskfromCompass
  (params (sideObjective :type PW%20Side%20Objective%20Object%20Reference))
  (Default|RemoveCompassLocation (Variables|Default|GetCompassHUD) (Variables|/Script/PROJECT_WEST.PW_SideObjective|Get_poiArea sideObjective)))