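; BP_GlassDestructable is a breakable glass actor that shatters when its health component reports death.
; On the death event, Break swaps the normal mesh for a newly added geometry collection and applies a constant-falloff radial impulse from the actor's location.
; The material effect component then builds its mesh components and plays backward, and the actor destroys itself after a short delay.
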(event Custom|OnDeathGlobal_Event
  (params (OwnerActor :type Actor%20Object%20Reference) (DamageCauser :type Actor%20Object%20Reference) (DamageCauserController :type Controller%20Object%20Reference))
  (bind _pw_materialeffect (Variables|Default|GetPW_MaterialEffect))
  (if (not (Variables|Default|GetIsBroken))
    (CallFunction|Break (Variables|Default|GetNormalMesh) (Transformation|GetActorLocation) 2e+02 2.5e+05)
    (Class|PWMaterialEffectComponent|GenerateMeshComponents _pw_materialeffect)
    (Class|PWMaterialEffectComponent|ActivateEffect _pw_materialeffect "ED_Backward")
    (Utilities|FlowControl|Delay 5.0)
    (Actor|DestroyActor)))

(event EventBeginPlay
  (EventDispatchers|AssignOnDeathGlobal (Variables|Default|GetPW_Health) (delegate Custom|OnDeathGlobal_Event)))

(fn ConstructionScript)

(fn Break
  (params (Normal%20Mesh :type Actor%20Component%20Object%20Reference) (Origin :type Vector) (Radius :type Float%20%28single-precision%29) (Strength :type Float%20%28single-precision%29))
  (Components|DestroyComponent Normal%20Mesh)
  (bind _returnvalue (AddComponent|AddGeometryCollectionComponent false))
  (Physics|AddRadialImpulse _returnvalue Origin Radius Strength "RIF_Constant" false)
  (Variables|Default|SetIsBroken true)
  (return _returnvalue))