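; Target location marker VFX Blueprint, filed under the Scorpion bounty's Steam Stinger Sky Barrage effects.
; Tick spins the root component around yaw by a fixed step per frame, so the speed depends on frame rate.
; The construction script does nothing, as its dynamic material and opacity setup for the star-target meshes and decals is left disconnected.
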(event EventBeginPlay)

(event Collision|EventActorBeginOverlap
  (params (OtherActor :type Actor%20Object%20Reference)))

(event EventTick
  (params (DeltaSeconds :type Float%20%28single-precision%29))
  (Transformation|AddLocalRotation (Variables|Default|GetDefaultSceneRoot) (Math|Rotator|MakeRotator 0.0 0.0 1.0) false false))

(fn ConstructionScript
  (Utilities|FlowControl|Sequence))