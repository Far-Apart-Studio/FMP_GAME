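; Player controller for Project West that wires gameplay events to the player's HUD, notifications and pop-up screens.
; When the player state is set, it binds loading screen, tutorial, item pickup and money events, then sets up notification, side objective and compass components, delayed on authority.
; Handlers show a data-table-driven loading screen, pickup and tutorial pop-ups, and the currency display.
; Helper functions toggle overall UI visibility and show a welcome note.
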(event Custom|Set%20Up%20Others
  (Default|SetUp (Variables|Default|GetBP_NotificationEvent))
  (Default|StartUp (Variables|Default|GetBP_SideObjUIHandler))
  (Default|SetUp (Variables|Default|GetBP_CompassLocator))
  (Development|PrintString "loadedddddddddd" true true "(R=0.000000,G=0.660000,B=1.000000,A=1.000000)" 1e+01))

(event Custom|Client%20Posses
  (Utilities|FlowControl|Delay 2.0)
  (Default|SetUp (Variables|Default|GetBP_NotificationEvent))
  (Default|StartUp (Variables|Default|GetBP_SideObjUIHandler))
  (Default|SetUp (Variables|Default|GetBP_CompassLocator)))

(event EventBeginPlay)

(event EventOnPlayerStateSet
  (EventDispatchers|AssignOnLoadingScreenTriggered (EventDispatchers|CreateEvent :!event OnLoadingScreenTriggered))
  (EventDispatchers|AssignOnTutorialInfoTriggered (EventDispatchers|CreateEvent :!event OnTutorialInfoTriggered))
  (CallFunction|AssignPickUpEvent)
  (CallFunction|AssignCurrecyChangedEvent)
  (Networking|SwitchHasAuthority
    (:Authority
      (Utilities|FlowControl|Delay 2.0)
      (CallFunction|SetUpOthers))
    (:Remote
      (CallFunction|SetUpOthers))))

(event EventPossess
  (params (PossessedPawn :type Pawn%20Object%20Reference)))

(fn ConstructionScript)

(fn OnLoadingScreenTriggered
  (params (levelData :type Map%20Data%20Entry%20Structure))
  (bind _returnvalue (UserInterface|CreateWidget "/Game/Project_West/UI/LoadingScreen/WB_LoadingScreen.WB_LoadingScreen_C"))
  (UserInterface|Viewport|AddtoViewport _returnvalue 0)
  (bind _returnvalue_2 (Utilities|GetDataTableRow "/Game/Project_West/Maps/Main_Maps/MapDateTable.MapDateTable" (Utilities|String|StringToName (._id levelData)))
    (:then
      (Default|SetInfo _returnvalue (._mapName (Utilities|Struct|BreakMapDataTable _returnvalue_2)) (._icon (Utilities|Struct|BreakMapDataTable _returnvalue_2))))))

(fn ToggleUIVisiblity
  (params (InVisibility :type ESlateVisibility%20Enum :default "Visible"))
  (Widget|SetVisibility (Variables|Default|Get_characterOverlayWidget) InVisibility)
  (Default|ToggleVisibility (Variables|Default|GetBP_SideObjUIHandler) InVisibility)
  (Default|ToggleVisibility (Variables|Default|GetBP_CompassLocator) InVisibility))

(fn OnTutorialInfoTriggered
  (params (info :type Info%20Entry%20Structure))
  (Default|DisplayTutorialPopUp (Variables|Default|GetBP_NotificationEvent) info))

(fn AssignPickUpEvent
  (EventDispatchers|BindEventtoOnItemPickup (Actor|GetComponentbyClass (Pawn|GetControlledPawn) "/Script/PROJECT_WEST.PW_InventoryHandler") (EventDispatchers|CreateEvent :!event OnItemPickUp)))

(fn OnItemPickUp
  (params (itemObject :type PW%20Item%20Object%20Object%20Reference))
  (bind _bp_notificationevent (Variables|Default|GetBP_NotificationEvent))
  (Default|DisplayPickUpNotification _bp_notificationevent "1" (Variables|/Script/PROJECT_WEST.PW_ItemObject|Get_itemIcon itemObject))
  (Default|DisplayTutorialPopUp _bp_notificationevent (Variables|/Script/PROJECT_WEST.PW_ItemObject|Get_infoDetails itemObject)))

(fn AssignCurrecyChangedEvent
  (EventDispatchers|BindEventtoOnMoneyValueChanged (EventDispatchers|CreateEvent :!event OnMoneyChanged)))

(fn OnMoneyChanged
  (params (info :type Integer))
  (bind _aspw_character_overlay_wbp_np (Utilities|Casting|CastToPW_CharacterOverlay_WBP_NP (Variables|Default|Get_characterOverlayWidget)))
  (Default|Display (Variables|/Game/Project_West/UI/HUD/PW_CharacterOverlay_WBP_NP.PW_CharacterOverlay_WBP_NP_C|GetWB_Currency _aspw_character_overlay_wbp_np)))

(fn DisplayWelcomeUI
  (bind _returnvalue (UserInterface|CreateWidget "/Game/Project_West/UI/Misc/WB_WelcomeNote.WB_WelcomeNote_C"))
  (UserInterface|Viewport|AddtoViewport _returnvalue 0))