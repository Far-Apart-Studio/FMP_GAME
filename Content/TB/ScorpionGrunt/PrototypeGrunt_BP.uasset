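; Prototype scorpion grunt enemy that roams, chases players, bites in melee and fires projectiles.
; Tick targets the nearest PW_Character on the navmesh for AIMoveTo, melee hitbox damage and chance-based shots, though range checks use player 0.
; Roam, chase, attack and shoot events have cooldowns or gates but rely on external triggers.
; A looping timer polls Health for death; the hit event plays a montage but subtracts zero health.
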(event Custom|Attack
  ;[1 1 1] Attack Event
  (CallFunction|MultiAttack))

(event Custom|MultiAttack
  ;[1 1 1] Attack Event
  (if (not (Variables|Default|GetDead))
    (if (not (Variables|Default|GetAttackCooldown))
      (Variables|Default|SetAttacking true)
      (Variables|Default|SetAttackCooldown true)
      (Variables|/Script/Engine.CharacterMovementComponent|SetMaxWalkSpeed (Variables|Character|GetCharacterMovement) 5.8e+02)
      (Animation|PlayAnimMontage "/Game/TB/PrototypeAttack.PrototypeAttack" 1.0 "None")
      (Utilities|FlowControl|Delay 0.3)
      (if (Collision|IsOverlappingActor (Variables|Default|GetPlayerAttackHitbox) (Variables|Default|GetClosestPlayerAI) :!class /Script/Engine.PrimitiveComponent)
        (Game|Damage|ApplyDamage (Variables|Default|GetClosestPlayerAI) 3e+01 0 0)
        (Utilities|FlowControl|Delay 0.8)
        (Variables|Default|SetAttackCooldown false)
        (else
          (Utilities|FlowControl|Delay 0.8)
          (Variables|Default|SetAttackCooldown false)))
      (Variables|/Script/Engine.CharacterMovementComponent|SetMaxWalkSpeed (Variables|Character|GetCharacterMovement) 675.0))))

(event Custom|MultiHit
  ;[1 1 1] Hit By Player
  (Variables|Default|SetHealth (- (Variables|Default|GetHealth) 0.0))
  (Animation|Montage|PlayMontage (Variables|Character|GetMesh) "/Game/TB/AM_ScorpionHit.AM_ScorpionHit"))

(event Custom|RandomRoam
  ;[1 1 1] Random Roaming
  (Utilities|FlowControl|DoOnce false
    (:Completed
      (AI|AIMoveTo self (.RandomLocation (AI|Navigation|GetRandomReachablePointinRadius (Transformation|GetActorLocation) 3e+03 0 0)) 0 5.0 false
        (:OnSuccess
          (Utilities|FlowControl|Delay (Math|Random|RandomFloatinRange 8.0 12.0))
          (if (not (Variables|Default|GetChasing))
            (CallFunction|Reset)
            (CallFunction|RandomRoam)))))))

(event Custom|Reset
  ;[1 1 1] Random Roaming
  (Utilities|FlowControl|DoOnce false) ; enters at Reset
)

(event Custom|AliveCheck
  ;[1 1 1] Alive Checking/Dying
  (if (<= (Variables|Default|GetHealth) 0.0)
    (Pawn|Components|CharacterMovement|DisableMovement (Variables|Character|GetCharacterMovement))
    (Utilities|FlowControl|DoOnce false
      (:Completed
        (Components|Animation|PlayAnimation (Variables|Character|GetMesh) "/Game/ExternalAssets/Scorpio/Animations/Anim_Scorpio_Death.Anim_Scorpio_Death" false)
        (Utilities|Time|ClearandInvalidateTimerbyHandle (stale EventBeginPlay _returnvalue))
        (Variables|Default|SetDead true)))))

(event Custom|MoveToPlayers
  ;[1 1 1] Move to player/Get players location
  (if (not (Variables|Default|GetDead))
    (if (Variables|Default|GetChasing)
      (AI|AIMoveTo (Class|PawnMovementComponent|GetPawnOwner (Variables|Character|GetCharacterMovement)) "0, 0, 0" (Variables|Default|GetClosestPlayerAI) 5.0 false
        (:OnSuccess
          _)
        (:OnFail
          _))
      (CallFunction|Reset))))

(event Custom|HitByPlayer
  ;[1 1 1] Hit By Player
  (CallFunction|MultiHit))

(event Custom|PlayerLocation
  ;[1 1 1] Move to player/Get players location
  (if (not (Variables|Default|GetDead))
    (if (Variables|Default|GetChasing)
      (Variables|Default|SetCurrentPlayerLocation (Transformation|GetActorLocation (Variables|Default|GetClosestPlayerAI))))))

(event Custom|ShootAttack
  ;[1 1 1] Shooting
  (CallFunction|DistanceCheck)
  (if (Variables|Default|GetRangedAttackDistance)
    (CallFunction|MultiShoot)))

(event Custom|MultiShoot
  ;[1 1 1] Shooting
  (if (not (Variables|Default|GetDead))
    (CallFunction|Shooting)
    (Animation|Montage|PlayMontage (Variables|Character|GetMesh) "/Game/TB/AM_ScorpionShootAttack.AM_ScorpionShootAttack"
      (:then
        (Utilities|FlowControl|Delay 5.0)
        (Variables|Default|SetShootingCD false)))))

(event EventTick
  (params (DeltaSeconds :type Float%20%28single-precision%29))
  ;[1 1 1] CheckingClosestPlayers
  (if (not (Variables|Default|GetDead))
    (bind _onnavmesh (CallFunction|GetActorsonNavmesh))
    (for (_array_element _array_index) _onnavmesh
      (if (== _array_index 0)
        (Variables|Default|SetCurrentClosestDistance (Transformation|GetDistanceTo self _array_element))
        (Variables|Default|SetClosestPlayerAI _array_element)
        (elif (< (Transformation|GetDistanceTo self _array_element) (Variables|Default|GetCurrentClosestDistance))
          (Variables|Default|SetCurrentClosestDistance (Transformation|GetDistanceTo self _array_element))
          (Variables|Default|SetClosestPlayerAI _array_element))))))

(event EventBeginPlay
  ;[1 1 1] Alive Checking/Dying
  (bind _returnvalue (Utilities|Time|SetTimerbyEvent (delegate Custom|AliveCheck) 0.01 true)))

(fn ConstructionScript)

(fn Shooting
  (bind _scene (Variables|Default|GetScene))
  (bind _returnvalue (Transformation|GetWorldLocation _scene))
  (if (not (Variables|Default|GetDead))
    (if (Variables|Default|GetChasing)
      (if (not (Variables|Default|GetShootingCD))
        (if (> (Math|Random|RandomFloatinRange 1.0 1e+02) 97.0)
          (Variables|Default|SetShootingCD true)
          (Game|SpawnActorfromClass "/Game/TB/BP_PrototypeAIProjectile.BP_PrototypeAIProjectile_C" (Math|Transform|MakeTransform _returnvalue (Math|Rotator|FindLookatRotation _returnvalue (Transformation|GetActorLocation (Variables|Default|GetClosestPlayerAI))) "1.000000,1.000000,1.000000") "Undefined" "MultiplyWithRoot" 0 0))))))

(fn DistanceCheck
  (bind _aspw_character (Utilities|Casting|CastToPW_Character (Game|GetPlayerCharacter 0)))
  (if (> (Transformation|GetDistanceTo _aspw_character) 6e+02)
    (Variables|Default|SetRangedAttackDistance true)
    (else
      (Variables|Default|SetRangedAttackDistance false))))

(fn GetActorsonNavmesh
  (bind _actorarray (LocalVariables|GetActorArray))
  (bind _outactors (Actor|GetAllActorsOfClass "/Script/PROJECT_WEST.PW_Character"))
  (for _array_element _outactors
    (if (AI|IsValidAILocation (Transformation|GetActorLocation _array_element))
      (Utilities|Array|Add _actorarray _array_element)))
  (return _actorarray))